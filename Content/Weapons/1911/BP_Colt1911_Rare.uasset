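; Rare Colt 1911 weapon variant that adds a visual buff effect while its owning player's rage is active.
; On BeginPlay it runs the parent logic, then binds to the owning NaziZombieCharacter's rage used and finished events, only when that character is locally controlled.
; Rage use attaches a particle emitter to the first-person mesh root, and rage finish detaches and destroys it.
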(event Custom|OnRageUsed_Event_0
  (bind _returnvalue (Effects|SpawnEmitterAttached "/Game/Weapons/WeaponEffects/Cascade/Particles/P_Colt1911_RageBuff.P_Colt1911_RageBuff" (Variables|/Script/WorldAtWar.CharacterBase|GetMesh1P (Variables|Default|GetPlayer)) "root" "0,100.000000, 0" "0,90.000000, 0" "1.000000,1.000000,1.000000" "SnapToTarget"))
  (Variables|Default|SetEmitter _returnvalue))

(event Custom|OnRageFinished_Event_0
  (Transformation|DetachFromComponent (Variables|Default|GetEmitter) "KeepRelative" "KeepRelative" "KeepRelative" true)
  (Components|DestroyComponent (Variables|Default|GetEmitter)))

(event EventBeginPlay
  (|CallParentFunction)
  (bind _asbp_nazi_zombie_character (Utilities|Casting|CastToBP_NaziZombieCharacter (Components|GetOwner)))
  (if (Pawn|IsLocallyControlled _asbp_nazi_zombie_character)
    (bind _output_get (Variables|Default|SetPlayer _asbp_nazi_zombie_character))
    (EventDispatchers|AssignOnRageUsed _output_get (delegate Custom|OnRageUsed_Event_0))
    (EventDispatchers|AssignOnRageFinished (Variables|Default|GetPlayer) (delegate Custom|OnRageFinished_Event_0))))

(fn ConstructionScript)