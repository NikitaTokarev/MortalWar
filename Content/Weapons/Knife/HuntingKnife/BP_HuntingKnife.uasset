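; Hunting knife weapon for the Nazi Zombie mode that lets its owner absorb health from knifed enemies.
; On the server, BeginPlay binds to the owning player state's knifing event to drive Absorption.
; When the player is below max health or infected, Absorption restores a small amount of health and ends any infection.
; A client event then plays a sound and, after a short delay, attaches particles to the slain enemy's chest.
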(event Custom|Absorption
  (params (SlainEnemy :type Zombie%20Base%20Object%20Reference))
  (if (CallFunction|NeedAbsorption)
    (Class|NaziZombieCharacter|RecoveryHealth (Variables|Default|GetPlayer) 7.5)
    (if (Variables|/Script/WorldAtWar.CharacterBase|GetbIsInfected (Variables|Default|GetPlayer))
      (Class|NaziZombieCharacter|DiseaseFinished (Variables|Default|GetPlayer)))
    (CallFunction|ClientPlayEffect SlainEnemy)))

(event Custom|Client_PlayEffect
  (params (SlainEnemy :type Zombie%20Base%20Object%20Reference))
  (Audio|PlaySoundatLocation "/Game/Audio/WeaponSounds/Knife/S_HuntingKnife_Absorption.S_HuntingKnife_Absorption" (Transformation|GetActorLocation) "0, 0, 0" 1.0 1.0 0.0 0 0 0)
  (Utilities|FlowControl|Delay 0.2)
  (Effects|SpawnEmitterAttached "/Game/Weapons/WeaponEffects/Cascade/Particles/P_HuntingKnife_Absorption.P_HuntingKnife_Absorption" (Variables|/Script/Engine.Character|GetMesh SlainEnemy) (Class|ZombieBase|GetChestBone SlainEnemy) "0, 0, 0" "0, 0, 0" "0.300000,0.300000,0.300000" "SnapToTarget"))

(event EventBeginPlay
  (|CallParentFunction)
  (Networking|SwitchHasAuthority
    (:Authority
      (bind _asbp_nazi_zombie_character (Utilities|Casting|CastToBP_NaziZombieCharacter (Components|GetOwner)))
      (bind _output_get (Variables|Default|SetPlayer _asbp_nazi_zombie_character))
      (bind _asbp_nazi_zombie_player_state (Utilities|Casting|CastToBP_NaziZombiePlayerState (Variables|/Script/Engine.Pawn|GetPlayerState _output_get)))
      (EventDispatchers|AssignOnKnifing _asbp_nazi_zombie_player_state (EventDispatchers|CreateEvent :!event Custom|Absorption)))))

(fn ConstructionScript)

(fn NeedAbsorption
  (bind _player (Variables|Default|GetPlayer))
  (return (or (not (Math|Float|NearlyEqual(Float) (Variables|/Script/WorldAtWar.NaziZombieCharacter|GetHealth _player) (Variables|/Script/WorldAtWar.NaziZombieCharacter|GetMaxHealth _player) 1e-06)) (Variables|/Script/WorldAtWar.CharacterBase|GetbIsInfected (Variables|Default|GetPlayer)))))