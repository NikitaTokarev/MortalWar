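; Rare STG44 weapon variant for the Nazi zombie character, adding a chance for hits to ricochet.
; On BeginPlay, only the authority caches the owning character's first-person camera and binds to the weapon hit event.
; Each hit has an even chance to call CalculateRicochet with the struck enemy, hit location and camera forward vector.
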(event Custom|OnWeaponHit_Event_0
  (params (TargetEnemy :type Zombie%20Base%20Object%20Reference) (HitLocation :type Vector))
  (if (Math|Random|RandomBoolwithWeight 0.5)
    (Class|WeaponBase|CalculateRicochet TargetEnemy HitLocation (Math|Vector|GetForwardVector (Variables|Default|GetPlayerCamera)))))

(event EventBeginPlay
  (|CallParentFunction)
  (Networking|SwitchHasAuthority
    (:Authority
      (bind _asnazi_zombie_character (Utilities|Casting|CastToNaziZombieCharacter (Components|GetOwner)))
      (Variables|Default|SetPlayerCamera (Variables|/Script/WorldAtWar.CharacterBase|GetFirstPersonCameraComponent _asnazi_zombie_character))
      (EventDispatchers|AssignOnWeaponHit (delegate Custom|OnWeaponHit_Event_0)))))

(fn ConstructionScript)