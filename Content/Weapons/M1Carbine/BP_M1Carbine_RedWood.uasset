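; M1 Carbine "RedWood" weapon variant that grants a temporary bonus-damage buff when its owner scores a headshot while holding it.
; On authority it binds to the player state's headshot event; repeat headshots restart the buff timer rather than stacking damage.
; Activation triggers client-side sound, ping effect and weapon tint through a dynamic material instance.
; Deactivation removes the bonus and resets the material parameters.
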(event Custom|ActivateHeadshotBuff
  (if (== (Class|CharacterBase|GetCurrentWeapon (Variables|Default|GetPlayer)) self)
    (if (Utilities|Time|IsTimerActivebyHandle (Variables|Default|GetTH_HeadshotBuff))
      (Utilities|Time|ClearandInvalidateTimerbyHandle (Variables|Default|GetTH_HeadshotBuff))
      (else
        (Class|WeaponBase|AddBonusDamage 35.0)))
    (bind _returnvalue (Utilities|Time|SetTimerbyEvent (EventDispatchers|CreateEvent :!event Custom|DeactivateHeadshotBuff) 6.5))
    (Variables|Default|SetTH_HeadshotBuff _returnvalue)
    (CallFunction|ClientPlayBuffEffects)))

(event Custom|Client_PlayBuffEffects
  (Utilities|FlowControl|Delay 0.25)
  (Audio|PlaySoundatLocation "/Game/Audio/WeaponSounds/Fire/S_Rifle_HeadshotBuff.S_Rifle_HeadshotBuff" (Transformation|GetActorLocation) "0, 0, 0" 1.0 1.0 0.0 0 0 0)
  (Rendering|Material|SetVectorParameterValue (Variables|Default|GetMI_WeaponMat) "HeadStotBuff_BaseColor" "(R=1.000000,G=0.250854,B=0.000000,A=1.000000)" :!class /Script/Engine.MaterialInstanceDynamic)
  (Rendering|Material|SetVectorParameterValue (Variables|Default|GetMI_WeaponMat) "HeadshotBuff_Emissive" "(R=0.000000,G=0.000844,B=0.001000,A=1.000000)" :!class /Script/Engine.MaterialInstanceDynamic)
  (Components|Activation|Activate (Variables|Default|GetP_Health_Player_Buff_Ping_01) true))

(event Custom|DeactivateHeadshotBuff
  (Class|WeaponBase|AddBonusDamage -35.0)
  (Utilities|Time|ClearandInvalidateTimerbyHandle (Variables|Default|GetTH_HeadshotBuff))
  (Rendering|Material|SetVectorParameterValue (Variables|Default|GetMI_WeaponMat) "HeadStotBuff_BaseColor" "(R=1.000000,G=1.000000,B=1.000000,A=1.000000)" :!class /Script/Engine.MaterialInstanceDynamic)
  (Rendering|Material|SetVectorParameterValue (Variables|Default|GetMI_WeaponMat) "HeadshotBuff_Emissive" "(R=0.000000,G=0.000000,B=0.000000,A=1.000000)" :!class /Script/Engine.MaterialInstanceDynamic))

(event EventBeginPlay
  (bind _weaponmesh (Variables|Default|GetWeaponMesh))
  (|CallParentFunction)
  (bind _returnvalue (Rendering|Material|CreateDynamicMaterialInstance _weaponmesh 0 (Rendering|Material|GetMaterial _weaponmesh 0) "None" :!class /Script/Engine.PrimitiveComponent))
  (Variables|Default|SetMI_WeaponMat _returnvalue)
  (Networking|SwitchHasAuthority
    (:Authority
      (bind _asbp_nazi_zombie_character (Utilities|Casting|CastToBP_NaziZombieCharacter (Components|GetOwner)))
      (bind _output_get (Variables|Default|SetPlayer _asbp_nazi_zombie_character))
      (bind _asbp_nazi_zombie_player_state (Utilities|Casting|CastToBP_NaziZombiePlayerState (Variables|/Script/Engine.Pawn|GetPlayerState _output_get)))
      (EventDispatchers|AssignOnHeadshot _asbp_nazi_zombie_player_state (EventDispatchers|CreateEvent :!event Custom|ActivateHeadshotBuff)))))

(fn ConstructionScript)