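; BP_AncientBook is an examinable book in the Sun Temple level that shows a touch prompt and can burn away.
; BeginPlay sets the prompt text and creates a dynamic material instance on the mesh.
; The BURN event starts particles and fire sound, then a looping timer gradually lowers the material's OpacityMask parameter.
; Near zero, it clears the timer, fades the sound out and sets a short lifespan to remove the actor.
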(event Custom|BURN
  (Components|Activation|Activate (Variables|Default|GetParticleSystem) false)
  (Audio|Components|Audio|FadeIn (Variables|Default|GetS_Fire) 2.0 1.0 0.0 "Linear" :!class /Script/Engine.AudioComponent)
  (bind _returnvalue (Utilities|Time|SetTimerbyEvent (delegate Custom|Burning) 0.1 true))
  (Variables|Default|SetTH_Burning _returnvalue))

(event Custom|Burning
  (bind _returnvalue (Rendering|Material|GetScalarParameterValue (Variables|Default|GetMI_Base) "OpacityMask" :!class /Script/Engine.MaterialInstanceDynamic))
  (Rendering|Material|SetScalarParameterValue (Variables|Default|GetMI_Base) "OpacityMask" (- _returnvalue 0.002) :!class /Script/Engine.MaterialInstanceDynamic)
  (if (Math|Float|NearlyEqual(Float) (- _returnvalue 0.002) 0.0 0.05)
    (Utilities|Time|ClearandInvalidateTimerbyHandle (Variables|Default|GetTH_Burning))
    (Audio|Components|Audio|FadeOut (Variables|Default|GetS_Fire) 2.0 0.0 "Linear" :!class /Script/Engine.AudioComponent)
    (Actor|SetLifeSpan 2.5)))

(event EventBeginPlay
  (bind _meshcomp (Variables|Default|GetMeshComp))
  (|CallParentFunction)
  (Variables|Default|SetUIMessage (Utilities|Text|MakeLiteralText "Two-finger touch to examine the mysterious book"))
  (bind _returnvalue (Rendering|Material|CreateDynamicMaterialInstance _meshcomp 0 (Rendering|Material|GetMaterial _meshcomp 0) "None" :!class /Script/Engine.PrimitiveComponent))
  (Variables|Default|SetMI_Base _returnvalue))

(fn ConstructionScript)