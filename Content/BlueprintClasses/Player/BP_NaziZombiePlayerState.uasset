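; Player state for the Nazi Zombie game that exposes a player's name data, points, final score and battle statistics.
; Three seconds after BeginPlay, the authority copies PlayerNames from the game instance into the state through the SetPlayerNames event.
; Getter functions wrap GetPoints, GetTotalScore and GetBattleStats, splitting the stats into kills, headshots, knifings and points.
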(event Custom|SetPlayerNames
  (params (PlayerNames :type Array%20of%20Strings))
  (Variables|Default|SetPlayerNames PlayerNames))

(event EventBeginPlay
  (Utilities|FlowControl|Delay 3.0)
  (Networking|SwitchHasAuthority
    (:Authority
      (bind _asbp_nazi_zombie_game_instance_base (Utilities|Casting|CastToBP_NaziZombieGameInstanceBase (Game|GetGameInstance)))
      (Variables|Default|SetPlayerNames (Variables|/Game/BlueprintClasses/BP_NaziZombieGameInstanceBase.BP_NaziZombieGameInstanceBase_C|GetPlayerNames _asbp_nazi_zombie_game_instance_base))
      (CallFunction|SetPlayerNames (Variables|Default|GetPlayerNames)))))

(fn ConstructionScript)

(fn GetBattleStatistics
  (bind (_reskills _resheadshots _resknifings _respoints) (Class|NaziZombiePlayerState|GetBattleStats))
  (return _reskills _resheadshots _resknifings _respoints))

(fn GetFinalScore
  (return (Class|NaziZombiePlayerState|GetTotalScore)))

(fn GetPlayerNames
  (return (Variables|Default|GetPlayerNames)))

(fn GetPlayerPoints
  (return (Class|NaziZombiePlayerState|GetPoints)))