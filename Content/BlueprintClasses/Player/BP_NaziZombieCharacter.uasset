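; First-person player character for the mobile Nazi zombie shooter, handling touch look, action buttons, interaction feedback and damage feedback.
; When locally controlled, it binds inherited health, rage, death and interaction events and loads sensitivity and skin color from the PlayerInfo save.
; A full rage bar unlocks Rage mode, which offline slows global time while speeding up the player.
; Death tilts the camera, then offers a leaderboard entry for qualifying scores or shows Game Over.
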(event Custom|ActionButtonPressed_1_1
  (params (Action :type E_Actions%20Enum :default "NewEnumerator0"))
  ;[0.2056 0.3352 1 1 32] Input
  (switch Utilities|FlowControl|Switch|SwitchonE_Actions Action
    (:NewEnumerator1
      (Class|CharacterBase|OnFire))
    (:NewEnumerator2
      (Class|NaziZombieCharacter|OnReload))
    (:NewEnumerator3
      (if (Variables|Default|GetbIsAiming)
        (Class|CharacterBase|OnAimingEnd)
        (else
          (Class|CharacterBase|OnAimingStart))))
    (:NewEnumerator4
      (Class|CharacterBase|SwitchNextWeapon false))
    (:NewEnumerator5
      (Class|NaziZombieCharacter|OnKnifeAttack))
    (:NewEnumerator6
      (Character|Jump))))

(event Custom|PlayDeathAnimation
  (bind _returnvalue (Pawn|GetControlRotation :!class /Script/Engine.Pawn))
  ;[1 0.03435 0 1 24] Death
  (Pawn|SetControlRotation (Pawn|GetController) (Math|Rotator|MakeRotator (+ (.roll _returnvalue) 0.25) (.pitch _returnvalue) (.yaw _returnvalue))))

(event Custom|OnDeathEvent
  ;[1 0.03435 0 1 24] Death
  (EventDispatchers|UnbindallEventsfromOnHealthChanged)
  (Utilities|Time|SetTimerbyEvent (EventDispatchers|CreateEvent :!event Custom|PlayDeathAnimation) 0.01 true)
  (Viewport|RemoveAllWidgets)
  (CallFunction|GameOver)
  (bind _outactors (Actor|GetAllActorsOfClass "/Game/BlueprintClasses/Zombies/ZombieClasses/BP_ZombieBase.BP_ZombieBase_C"))
  (for _array_element _outactors
    (if (Math|Random|RandomBoolwithWeight 0.7)
      (Class|BPIEnemyBase|ShutdownSound(Message) _array_element))))

(event Custom|OnRageFinished_Event_0
  ;[1 1 1 1 24] On Rage Finished
  (CallFunction|SetUsualMode)
  (Variables|Default|SetbRageEnabled false))

(event Custom|OnRageChanged_Event_0
  (params (NewRage :type Float%20%28single-precision%29))
  ;[1 0.5774 0 1 24] On Rage Changed
  (if (and (== NewRage (Variables|Default|GetMaxRage)) (not (Variables|Default|GetbIsRage)))
    (Variables|Default|SetbRageEnabled true)
    (Audio|PlaySound2D "/Game/Audio/Interface/S_EnterGame.S_EnterGame" 7.5 1.0 0.0 0 0)
    (Default|CallOnRageBarFulled)))

(event Custom|SaveMutantIsKnown
  (bind _sg_playerinfo (Variables|Default|GetSG_PlayerInfo))
  (Default|SetMutantIsKnown _sg_playerinfo)
  (SaveGame|SaveGametoSlot _sg_playerinfo "PlayerInfo"))

(event Custom|CustomEvent_2
  (Variables|Default|SetbDontWatchBack false))

(event Custom|OnInteracted_Event_0
  (params (InteractableObject :type Interactable%20Base%20Object%20Reference))
  (Variables|Default|SetbDontWatchBack true)
  (Utilities|Time|SetTimerbyEvent (delegate Custom|CustomEvent_2) 0.33)
  (CallFunction|PlayInteractionSound InteractableObject))

(event Custom|ActivateBless_PunishingHand
  (bind _mesh1p (Variables|Default|GetMesh1P))
  (bind _mesh1p_2 (Variables|Default|GetMesh1P))
  (bind _returnvalue (Rendering|Material|CreateDynamicMaterialInstance _mesh1p 1 (Rendering|Material|GetMaterial _mesh1p 1) "None" :!class /Script/Engine.PrimitiveComponent))
  (Rendering|Material|SetVectorParameterValue _returnvalue "Color" "(R=0.709804,G=0.094118,B=0.094118,A=1.000000)" :!class /Script/Engine.MaterialInstanceDynamic)
  (bind _returnvalue_2 (Rendering|Material|CreateDynamicMaterialInstance _mesh1p_2 2 (Rendering|Material|GetMaterial _mesh1p_2 2) "None" :!class /Script/Engine.PrimitiveComponent))
  (Rendering|Material|SetVectorParameterValue _returnvalue_2 "Color" "(R=0.709804,G=0.094118,B=0.094118,A=1.000000)" :!class /Script/Engine.MaterialInstanceDynamic))

(event Custom|OnHealthChanged_Event_0
  (params (NewHealth :type Float%20%28single-precision%29))
  ;[0.3281 1 0.02473 1 24] On Health Changed
  (if (> NewHealth 0.0)
    (if (< NewHealth (Variables|Default|GetPreviousHealth))
      (Default|CallOnTakeDamage (- NewHealth (Variables|Default|GetPreviousHealth)))
      (Variables|Default|SetLastDamage (- NewHealth (Variables|Default|GetPreviousHealth)))
      (CameraShakes|StartCameraShake (Game|GetPlayerCameraManager 0) "/Game/BlueprintClasses/Player/BP_DamageCameraShake.BP_DamageCameraShake_C" 1.0 "CameraLocal" "0, 0, 0")
      (Variables|Default|SetPreviousHealth NewHealth)
      (if (Variables|Default|GetbIsInfected)
        (if (or (>= (Variables|Default|GetLastDamage) 5.0) (Math|Random|RandomBoolwithWeight 0.6))
          (Utilities|FlowControl|Delay 0.15 :!label _label)
          (CallFunction|PlayPainSound))
        (else
          (goto _label)))
      (else
        (Variables|Default|SetPreviousHealth NewHealth)))))

(event Custom|OnTouchSensivityChanged
  (params (NewTouchSensivity :type Float%20%28single-precision%29))
  ;[0.6779 0.5157 1 1 24] On Touch Sensivity Changed
  (Variables|Default|SetTouchSensivity NewTouchSensivity))

(event Custom|SimulateMoving
  ;[1 0.5829 0 1 32] ???No Animation???
  (if (not (Utilities|Time|IsValidTimerHandle (Variables|Default|GetTH_DownArms)))
    (bind _returnvalue (Utilities|Time|SetTimerbyEvent (delegate Custom|DownWeapon) 0.01 true))
    (Variables|Default|SetTH_DownArms _returnvalue)))

(event Custom|DownWeapon
  (bind _mesh1p (Variables|Default|GetMesh1P))
  (bind _relativerotation (Variables|/Script/Engine.SceneComponent|GetRelativeRotation _mesh1p))
  (bind (_roll _pitch _yaw) (Math|Rotator|BreakRotator _relativerotation))
  ;[1 0.5829 0 1 32] ???No Animation???
  (Transformation|SetRelativeRotation _mesh1p (Math|Rotator|MakeRotator (Math|Interpolation|FInterpTo _roll (select (CallFunction|CurrentWeaponIsCarbine) 25.0 2e+01) (Utilities|Time|GetWorldDeltaSeconds) 25.0) _pitch _yaw) false false))

(event Custom|StopSimulateMoving
  ;[1 0.5829 0 1 32] ???No Animation???
  (Utilities|Time|ClearandInvalidateTimerbyHandle (Variables|Default|GetTH_DownArms))
  (if (not (Math|Float|NearlyEqual(Float) (.Roll (Math|Rotator|BreakRotator (Variables|/Script/Engine.SceneComponent|GetRelativeRotation (Variables|Default|GetMesh1P)))) 0.0 1.1))
    (bind _returnvalue (Utilities|Time|SetTimerbyEvent (delegate Custom|UpWeapon) (select (CallFunction|CurrentWeaponIsCarbine) 0.0075 0.009) true))
    (Variables|Default|SetTH_UpArms _returnvalue)
    (Utilities|FlowControl|Delay 0.45)
    (Utilities|Time|ClearandInvalidateTimerbyHandle (Variables|Default|GetTH_UpArms))
    (Transformation|SetRelativeRotation (Variables|Default|GetMesh1P) "0,-90.000000, 0" false false)))

(event Custom|UpWeapon
  (bind _mesh1p (Variables|Default|GetMesh1P))
  (bind _relativerotation (Variables|/Script/Engine.SceneComponent|GetRelativeRotation _mesh1p))
  (bind (_roll _pitch _yaw) (Math|Rotator|BreakRotator _relativerotation))
  (bind _returnvalue (- _roll 1.0))
  ;[1 0.5829 0 1 32] ???No Animation???
  (if (Math|Float|NearlyEqual(Float) _returnvalue 0.0 0.5)
    (Utilities|Time|ClearandInvalidateTimerbyHandle (Variables|Default|GetTH_UpArms))
    (Transformation|SetRelativeRotation (Variables|Default|GetMesh1P) "0,-90.000000, 0" false false)
    (else
      (Transformation|SetRelativeRotation (Variables|Default|GetMesh1P) (Math|Rotator|MakeRotator _returnvalue _pitch _yaw) false false))))

(event Custom|OnInteractChanged_Event_0
  (params (InteractableObject :type Interactable%20Base%20Object%20Reference))
  (bind (_returnvalue _bisavailable _bisused _bspecialcolor _specialcolor) (CallFunction|GetInteractableInfo InteractableObject))
  (Default|CallOnInteractInfoChanged _returnvalue _bisavailable _bisused _bspecialcolor _specialcolor))

(event Custom|TryActivateRageMode
  (bind _returnvalue (Class|CharacterBase|GetCurrentWeapon))
  ;[0.2056 0.3352 1 1 32] Input
  (if (Math|Boolean|ANDBoolean (Variables|Default|GetbRageEnabled) (not (Variables|Default|GetbIsRage)) (Class|WeaponBase|GetCanFire _returnvalue) (not (Class|WeaponBase|GetIsReloading _returnvalue)))
    (if (Variables|Default|GetbIsInfected)
      (Class|NaziZombieCharacter|DiseaseFinished))
    (CallFunction|SetRageMode)
    (Audio|PlaySound2D "/Game/Audio/Game/S_RageStarted.S_RageStarted" 1.0 1.0 0.0 0 0)
    (Default|CallOnRageUsed)))

(event EventBeginPlay
  ;[1 0.4938 0 1 32] BeginPlay
  (|CallParentFunction)
  (if (Pawn|IsLocallyControlled)
    ;[0.934 0 1] Setup Local Bindings
    (EventDispatchers|AssignOnInteractChanged (delegate Custom|OnInteractChanged_Event_0))
    (EventDispatchers|AssignOnDeath (EventDispatchers|CreateEvent :!event Custom|OnDeathEvent))
    (EventDispatchers|AssignOnRageChanged (EventDispatchers|CreateEvent :!event Custom|OnRageChanged_Event_0))
    (EventDispatchers|AssignOnRageFinished (EventDispatchers|CreateEvent :!event Custom|OnRageFinished_Event_0))
    (CallFunction|LoadGamefromSlot)
    (EventDispatchers|AssignOnTouchSensivityChanged (Variables|Default|GetSG_PlayerInfo) (EventDispatchers|CreateEvent :!event Custom|OnTouchSensivityChanged))
    (EventDispatchers|AssignOnInteracted (delegate Custom|OnInteracted_Event_0))
    (|LoadSettings)
    (Utilities|FlowControl|Delay 2.0)
    (EventDispatchers|AssignOnHealthChanged (EventDispatchers|CreateEvent :!event Custom|OnHealthChanged_Event_0))
    (Variables|Default|SetPreviousHealth (Variables|Default|GetHealth))))

(event EventIncrementPlayerPoints
  (params (Amount :type Integer))
  (Class|NaziZombieCharacter|IncrementPoints Amount))

(event EventAddRecordtoLadder
  (params (Name :type String))
  (bind _sg_playerinfo (Variables|Default|GetSG_PlayerInfo))
  ;[1 1 1] Add Record To Ladder
  (bind _returnvalue (Class|BPIPlayerState|GetFinalScore(Message) (Variables|Default|GetPlayerState)))
  (bind _index (Class|BPISaveGame|AddRecordtoLadder(Message) _sg_playerinfo Name _returnvalue (CallFunction|GetMapDisplayName)))
  (SaveGame|SaveGametoSlot _sg_playerinfo "PlayerInfo")
  (bind _ladderrecords (Class|BPISaveGame|GetLadder(Message) (Variables|Default|GetSG_PlayerInfo)))
  (bind _returnvalue_2 (UserInterface|CreateWidget "/Game/UI/Game/GameOver/W_Ladder.W_Ladder_C" (Game|GetPlayerController 0) 0 _index true _ladderrecords))
  (UserInterface|Viewport|AddtoViewport _returnvalue_2 0))

(event Input|KeyboardEvents|K
  (params (Key :type Key%20Structure :default "None"))
  ;[0.2056 0.3352 1 1 32] Input
  (:Pressed
    (CallFunction|TryActivateRageMode)))

(event Input|TouchEvents|Touch1
  (params (Key :type Key%20Structure :default "None"))
  ;[0.2056 0.3352 1 1 32] Input
  (:Pressed
    (Variables|Default|SetbIsPressed true))
  (:Released
    (Variables|Default|SetbIsPressed false)))

(event Input|TouchEvents|InputTouch
  (params (Location :type Vector) (FingerIndex :type ETouchIndex%20Enum))
  ;[0.2056 0.3352 1 1 32] Input
  (:Pressed
    (switch Utilities|FlowControl|Switch|SwitchonETouchIndex FingerIndex
      (:Touch1
        _)
      (:Touch2
        (Utilities|ShouldRotate
          (:True
            _))))
    (Variables|Default|SetTouchLocation (Math|Conversions|ToVector2D(Vector) (/ Location 1e+01))))
  (:Moved
    (switch Utilities|FlowControl|Switch|SwitchonETouchIndex FingerIndex
      (:Touch1
        (CallFunction|RotateCamera (Math|Conversions|ToVector2D(Vector) (/ Location 1e+01)) :!label _label))
      (:Touch2
        (if (not (Variables|Default|GetbDontWatchBack))
          (goto _label))))))

(fn ConstructionScript)

(fn RotateCamera
  (params (Location :type Vector%202D%20Structure))
  (bind _output_get (LocalVariables|SetTouchDeltaMove (select (Variables|Default|GetbIsAiming) (/ (* (* (- (Variables|Default|GetTouchLocation) Location) -1.0) (Variables|Default|GetTouchSensivity)) 2.75) (* (* (- (Variables|Default|GetTouchLocation) Location) -1.0) (Variables|Default|GetTouchSensivity)))))
  (Pawn|Input|AddControllerYawInput (.X (Math|Vector2D|BreakVector2D _output_get)))
  (Pawn|Input|AddControllerPitchInput (.Y (Math|Vector2D|BreakVector2D _output_get)))
  (Variables|Default|SetTouchLocation Location)
  (return))

(fn CreateGameOverWidget
  (bind (_message _color) (CallFunction|GetGameOverMessageandColor))
  (bind _returnvalue (Class|BPIPlayerState|GetFinalScore(Message) (Variables|Default|GetPlayerState)))
  (bind _returnvalue_2 (UserInterface|CreateWidget "/Game/UI/Game/GameOver/W_GameOver.W_GameOver_C" (Game|GetPlayerController 0) _returnvalue (< (Utilities|Array|Length (Variables|/Script/Engine.GameStateBase|GetPlayerArray (Game|GetGameState))) 2) _message _color))
  (UserInterface|Viewport|AddtoViewport _returnvalue_2 0)
  (return))

(fn GameOver
  (Audio|PlaySound2D "/Game/Audio/Characters/Player/S_Character_Death.S_Character_Death" 1.0 1.0 0.0 0 0)
  (Components|Animation|SetAnimationMode (Variables|Default|GetMesh1P) "AnimationCustomMode")
  (CallFunction|GameFinished)
  (return))

(fn PlayPainSound
  (if (Variables|Default|GetbPlayPainSound)
    (Variables|Default|SetbPlayPainSound false)
    (Audio|PlaySound2D (.OutItem (Utilities|Array|Random (Variables|Default|GetPainSounds))) 1.0 1.0 0.0 0 0)
    (Utilities|Time|SetTimerbyFunctionName 0 "ResetPlayPainSound" 0.45)
    (return)))

(fn ResetPlayPainSound
  (Variables|Default|SetbPlayPainSound true)
  (return))

(fn LoadGamefromSlot
  (bind _returnvalue (SaveGame|LoadGamefromSlot "PlayerInfo"))
  (bind _assg_player_info (Utilities|Casting|CastToSG_PlayerInfo _returnvalue)
    (:then
      (Variables|Default|SetSG_PlayerInfo _assg_player_info)
      (return))
    (:CastFailed
      (return))))

(fn SetRageMode
  (if (Class|BlueprintFunctionLibraryMisc|IsOnline self)
    _
    (else
      (Utilities|Time|SetGlobalTimeDilation 0.2)
      (Variables|Default|SetCustomTimeDilation 3.5)))
  (Class|NaziZombieCharacter|EnableRageMode)
  (return))

(fn SetUsualMode
  (if (Class|BlueprintFunctionLibraryMisc|IsOnline self)
    _
    (else
      (Utilities|Time|SetGlobalTimeDilation 1.0)
      (Variables|Default|SetCustomTimeDilation 1.0)))
  (return))

(fn GetInteractableCost
  (params (Interactable :type Interactable%20Base%20Object%20Reference))
  (Utilities|IsValid Interactable
    (:Is%20Valid
      (return (Class|InteractableBase|GetCost Interactable)))
    (:Is%20Not%20Valid
      (return 0))))

(fn GetInteractableInfo
  (params (Interactable :type Interactable%20Base%20Object%20Reference))
  (Utilities|IsValid Interactable
    (:Is%20Valid
      (bind _asbp_wall_weapon_firearms (Utilities|Casting|CastToBP_WallWeapon_Firearms Interactable)
        (:then
          (Class|WallWeapon|ChangeUIMessage _asbp_wall_weapon_firearms))
        (:CastFailed
          _))
      (bind _points (Class|BPIPlayerState|GetPlayerPoints(Message) (Variables|Default|GetPlayerState)))
      (return (Class|InteractableBase|GetUIMessage Interactable) (>= _points (Class|InteractableBase|GetCost Interactable self)) (Class|InteractableBase|IsAlreadyUsed Interactable self) (Class|InteractableBase|HasSpecialColor Interactable) (Class|InteractableBase|GetSpecialColor Interactable)))
    (:Is%20Not%20Valid
      (return "" false false false ""))))

(fn CurrentWeaponIsCarbine
  (return (== (Utilities|GetClass (Class|CharacterBase|GetCurrentWeapon)) "/Game/Weapons/M1Carbine/BP_M1Carbine.BP_M1Carbine_C")))

(fn GetMapDisplayName
  (bind _returnvalue (Game|GetCurrentLevelName true))
  (bind _returnvalue_2 (Utilities|GetDataTableRow "/Game/Data/DT_MapInfo.DT_MapInfo" (Utilities|String|StringToName _returnvalue))
    (:then
      (return (Utilities|Struct|BreakS_MapInfo _returnvalue_2)))
    (:RowNotFound
      (return "Map"))))

(fn IsTrueMatch
  (bind _returnvalue (Class|BPIPlayerState|GetMissionState(Message) (Variables|Default|GetPlayerState)))
  (bind _returnvalue_2 (Game|GetCurrentLevelName true))
  (return (and (Utilities|Enum|NotEqual(Enum) _returnvalue_2 "TrainingMap") (Utilities|Enum|NotEqual(Enum) _returnvalue "NewEnumerator1"))))

(fn PlayInteractionSound
  (params (InteractableObject :type Interactable%20Base%20Object%20Reference))
  (bind _returnvalue (Utilities|GetClass InteractableObject))
  (if (Utilities|ClassIsChildOf _returnvalue "/Script/WorldAtWar.WallWeapon")
    (bind _bisavailable (CallFunction|GetInteractableInfo InteractableObject))
    (if _bisavailable
      (if (Utilities|ClassIsChildOf _returnvalue "/Script/WorldAtWar.WallWeapon_Firearms")
        (bind _asbp_wall_weapon_firearms (Utilities|Casting|CastToBP_WallWeapon_Firearms InteractableObject)
          (:then
            (if (CallFunction|ShouldPlayInterSound (Variables|/Script/WorldAtWar.WallWeapon_Firearms|GetWeaponClass _asbp_wall_weapon_firearms))
              (Audio|PlaySound2D "/Game/Audio/Game/S_EquipWeapon_Firearms.S_EquipWeapon_Firearms" 1.0 1.0 0.0 0 0)
              (return)
              (else
                (return))))
          (:CastFailed
            (return)))
        (else
          (Audio|PlaySound2D "/Game/Audio/Game/S_EquipWeapon_Melee.S_EquipWeapon_Melee" 1.0 1.0 0.0 0 0)
          (return)))
      (else
        (return)))
    (elif (Utilities|ClassIsChildOf _returnvalue "/Script/WorldAtWar.LootWeaponBase")
      (bind _asloot_weapon_base (Utilities|Casting|CastToLootWeaponBase InteractableObject)
        (:then
          (Audio|PlaySound2D (select (Class|LootWeaponBase|GetIsFirearms _asloot_weapon_base) "/Game/Audio/Game/S_EquipWeapon_Firearms.S_EquipWeapon_Firearms" "/Game/Audio/Game/S_EquipWeapon_Melee.S_EquipWeapon_Melee") 1.0 1.0 0.0 0 0)
          (return))
        (:CastFailed
          (return)))
      (else
        (return)))))

(fn GetGameOverMessageandColor
  (bind _playerstate (Variables|Default|GetPlayerState))
  (bind _returnvalue (Class|BPIPlayerState|GetGameOverMessage(Message) _playerstate))
  (bind _returnvalue_2 (Class|BPIPlayerState|GetMissionState(Message) _playerstate))
  (return _returnvalue (Utilities|Select :Index _returnvalue_2 :NewEnumerator0 "(R=1.000000,G=0.458824,B=0.000000,A=0.800000)" :NewEnumerator1 "(R=0.887500,G=0.000000,B=0.000000,A=0.800000)" :NewEnumerator2 "(R=0.023529,G=1.000000,B=0.274510,A=0.800000)")))

(fn GameFinished
  (if (Variables|Default|GetbIsInfected)
    (Class|NaziZombieCharacter|DiseaseFinished))
  (bind _ladderrecords (Class|BPISaveGame|GetLadder(Message) (Variables|Default|GetSG_PlayerInfo)))
  (bind _returnvalue (Class|BPIPlayerState|GetFinalScore(Message) (Variables|Default|GetPlayerState)))
  (if (and (CallFunction|IsTrueMatch) (> _returnvalue (Utilities|Struct|BreakS_LadderInfo (Utilities|Array|Get(acopy) _ladderrecords (Utilities|Array|LastIndex _ladderrecords)))))
    (bind _returnvalue_2 (Class|BPISaveGame|GetBusyNames(Message) (Variables|Default|GetSG_PlayerInfo)))
    (bind _returnvalue_3 (UserInterface|CreateWidget "/Game/UI/Game/GameOver/W_AddRecordToLadder.W_AddRecordToLadder_C" (Game|GetPlayerController 0) _returnvalue_2))
    (UserInterface|Viewport|AddtoViewport _returnvalue_3 0)
    (else
      (CallFunction|CreateGameOverWidget))))

(fn ShouldPlayInterSound
  (params (WeaponClass :type Weapon%20Base%20Class%20Reference))
  (LocalVariables|SetL_WeaponID (select (Utilities|ClassIsChildOf WeaponClass "/Game/Weapons/1911/BP_Colt1911.BP_Colt1911_C") "Colt1911" (select (Utilities|ClassIsChildOf WeaponClass "/Game/Weapons/M1Carbine/BP_M1Carbine.BP_M1Carbine_C") "M1Carbine" "STG44")))
  (Utilities|IsValid (Utilities|Array|Get(acopy) (Class|CharacterBase|GetWeaponsArray) (Utilities|Select :Index (LocalVariables|GetL_WeaponID) :Colt1911 0 :M1Carbine 1 :STG44 2))
    (:Is%20Valid
      (return (Class|NaziZombieCharacter|NeedAmmo (LocalVariables|GetL_WeaponID))))
    (:Is%20Not%20Valid
      (return true))))

(fn GetIsImmunetoEffects
  (return (Variables|Default|GetbIsImmuneToEffects)))

(fn SetIsImmunetoEffects
  (params (IsImmune :type Boolean))
  (Variables|Default|SetbIsImmuneToEffects IsImmune)
  (return))

(fn ActionButtonPressed
  (params (Action :type E_Actions%20Enum :default "NewEnumerator0"))
  (switch Utilities|FlowControl|Switch|SwitchonE_Actions Action
    (:NewEnumerator1
      (Class|CharacterBase|OnFire)
      (return (Class|WeaponBase|GetCanFire (Class|CharacterBase|GetCurrentWeapon))))
    (:NewEnumerator2
      (Class|NaziZombieCharacter|OnReload)
      (return true))
    (:NewEnumerator3
      (if (Variables|Default|GetbIsAiming)
        (Class|CharacterBase|OnAimingEnd)
        (else
          (Class|CharacterBase|OnAimingStart)))
      (return true))
    (:NewEnumerator4
      (Class|CharacterBase|SwitchNextWeapon true)
      (return true))
    (:NewEnumerator5
      (Class|NaziZombieCharacter|OnKnifeAttack)
      (return true))
    (:NewEnumerator6
      (Character|Jump)
      (return true))))

(fn GetCharacterIsDead
  (return (Class|NaziZombieCharacter|GetIsDead)))

(fn GetPlayerRef
  (return self))

(fn GetPlayerWeapon
  (return (Class|CharacterBase|GetCurrentWeapon)))