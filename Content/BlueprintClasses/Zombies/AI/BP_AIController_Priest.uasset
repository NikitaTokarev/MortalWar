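; AI controller for the Priest, an enemy that fights the player with melee attacks and minion summoning.
; UseAvailableSkill loops until player death, trying close-range melee, else choosing from a priority-weighted DataTable and firing the skill's event by timer name, re-queuing it after cooldown.
; Summons spawn buffed zombies at the nearest TargetPoints, with class odds and buff scaled by Priest health.
; Living minions unlock extra skills; BuffOne, BuffTwo and DoNothing are print-only placeholders.
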(event Custom|UseAvailableSkill
  (if (Variables|Default|GetbShouldContinue)
    (Utilities|TryMeleeAttack
      (:Continue
        (if (!= (Utilities|Array|Length (Variables|Default|GetSkills_RowNames)) 0)
          (Skills|GetNextSkill)
          (else
            (Utilities|FlowControl|Delay 0.5)
            (CallFunction|UseAvailableSkill)))))))

(event Custom|SummoningMinions
  (bind _priest (Variables|Default|GetPriest))
  ;[1 0.6098 0 1 32] Summoning Minions
  (Animation|Montage|MontagePlay (Default|GetAnimInstance (Variables|Default|GetPriest)) "/Game/BlueprintClasses/Zombies/Animations/Boss_Priest/AM_Priest_SummoningMinions.AM_Priest_SummoningMinions" 1.0 "MontageLength" 0.0 true)
  (Utilities|FlowControl|Delay 1.25)
  (bind _returnvalue (Skills|SummoningMinions|GetClosestSpawnPoints))
  (for _array_element _returnvalue
    (bind _returnvalue_2 (Game|SpawnActorfromClass (Skills|SummoningMinions|GetZombieClass) (Transformation|GetActorTransform (Utilities|Array|Get(acopy) (Variables|Default|GetZombieSpawnPoints) _array_element)) "AlwaysSpawn" _priest false _priest))
    (Utilities|Array|Add (Variables|Default|GetMinions) _returnvalue_2)
    (EventDispatchers|BindEventtoOnEnemyDeath _returnvalue_2 (EventDispatchers|CreateEvent :!event Custom|OnMinionDeath))
    (Class|ZombieBase|ActivateBuff _returnvalue_2 0.0 true (Skills|SummoningMinions|CalculateBuffStrength))
    (Effects|SpawnEmitteratLocation "/Game/InfinityBladeEffects/Effects/FX_Mobile/combat/P_AuraCircle_LeachTarget.P_AuraCircle_LeachTarget" (- (Transformation|GetActorLocation (Utilities|Array|Get(acopy) (Variables|Default|GetZombieSpawnPoints) _array_element)) "0, 0,85.000000")))
  (if (not (Variables|Default|GetbHasMinions))
    (Skills|AddSkillsBuffs)
    (Variables|Default|SetbHasMinions true))
  (Utilities|FlowControl|Delay 2.0)
  ;;[1 1 1] Skill Name !!!
  (bind _cooldown (Skills|RemoveUsedSkill "SummoningMinions"))
  (CallFunction|UseAvailableSkill)
  (Utilities|FlowControl|Delay _cooldown)
  (Utilities|Array|Insert (Variables|Default|GetSkills_RowNames) "SummoningMinions"))

(event Custom|OnMinionDeath
  (params (Enemy :type Zombie%20Base%20Object%20Reference))
  ;[1 0.6098 0 1 32] Summoning Minions
  (bind _asbp_zombie_base (Utilities|Casting|CastToBP_ZombieBase Enemy))
  (Utilities|Array|RemoveItem (Variables|Default|GetMinions) _asbp_zombie_base)
  (Utilities|Array|Add (Variables|Default|GetDeadMinions) _asbp_zombie_base)
  (Game|BindEventtoOnDestroyed _asbp_zombie_base (EventDispatchers|CreateEvent :!event Custom|OnMinionDestroyed))
  (if (== (Utilities|Array|Length (Variables|Default|GetMinions)) 0)
    (Variables|Default|SetbHasMinions false)
    (Skills|RemoveSkillsBuffs)))

(event Custom|DoNothing
  (Development|PrintString "Do Nothing" true true "(R=0.008488,G=0.000000,B=0.496875,A=1.000000)" 4.0)
  (Utilities|FlowControl|Delay 1.0)
  (bind _cooldown (Skills|RemoveUsedSkill "DoNothing"))
  (CallFunction|UseAvailableSkill)
  (Utilities|FlowControl|Delay _cooldown)
  (if (Variables|Default|GetbHasMinions)
    (Utilities|Array|Insert (Variables|Default|GetSkills_RowNames) "DoNothing" (Math|Random|RandomIntegerinRange 0 (Utilities|Array|LastIndex (Variables|Default|GetSkills_RowNames))))))

(event Custom|OnDeath_Event_0
  (Variables|Default|SetbShouldContinue false))

(event Custom|OnMinionDestroyed
  (params (DestroyedActor :type Actor%20Object%20Reference))
  ;[1 0.6098 0 1 32] Summoning Minions
  (bind _asbp_zombie_base (Utilities|Casting|CastToBP_ZombieBase DestroyedActor))
  (Utilities|Array|RemoveItem (Variables|Default|GetDeadMinions) _asbp_zombie_base))

(event Custom|BuffOne
  (Development|PrintString "Buff One" true true "(R=0.000000,G=0.160483,B=1.000000,A=1.000000)" 4.0)
  (Utilities|FlowControl|Delay 2.0)
  (bind _cooldown (Skills|RemoveUsedSkill "BuffOne"))
  (CallFunction|UseAvailableSkill)
  (Utilities|FlowControl|Delay _cooldown)
  (if (Variables|Default|GetbHasMinions)
    (Utilities|Array|Insert (Variables|Default|GetSkills_RowNames) "BuffOne" (Math|Random|RandomIntegerinRange 0 (Utilities|Array|LastIndex (Variables|Default|GetSkills_RowNames))))))

(event Custom|BuffTwo
  (Development|PrintString "Buff Two" true true "(R=1.000000,G=0.255271,B=0.000000,A=1.000000)" 4.0)
  (Utilities|FlowControl|Delay 2.0)
  (bind _cooldown (Skills|RemoveUsedSkill "BuffTwo"))
  (CallFunction|UseAvailableSkill)
  (Utilities|FlowControl|Delay _cooldown)
  (if (Variables|Default|GetbHasMinions)
    (Utilities|Array|Insert (Variables|Default|GetSkills_RowNames) "BuffTwo" (Math|Random|RandomIntegerinRange 0 (Utilities|Array|LastIndex (Variables|Default|GetSkills_RowNames))))))

(event EventBeginPlay
  (Utilities|FlowControl|Delay 1.35)
  (bind _asbp_priest (Utilities|Casting|CastToBP_Priest (Pawn|GetControlledPawn)))
  (Variables|Default|SetPriest _asbp_priest)
  (bind _asbp_nazi_zombie_character (Utilities|Casting|CastToBP_NaziZombieCharacter (Game|GetPlayerCharacter 0)))
  (bind _output_get (Variables|Default|SetPlayer _asbp_nazi_zombie_character))
  (EventDispatchers|AssignOnDeath _output_get (delegate Custom|OnDeath_Event_0))
  (bind _outactors (Actor|GetAllActorsOfClass "/Script/Engine.TargetPoint"))
  (Variables|Default|SetZombieSpawnPoints _outactors))

(event EventTick
  (params (DeltaSeconds :type Float%20%28single-precision%29))
  (for _array_element (Variables|Default|GetSkills_RowNames)
    (Development|PrintString (Utilities|String|ToString(Name) _array_element) true true "(R=0.000000,G=0.660000,B=1.000000,A=1.000000)" 0.0)))

(fn ConstructionScript)

(fn GetClosestSpawnPoints
  (bind _l_distances (LocalVariables|GetL_Distances))
  (bind _l_indexes (LocalVariables|GetL_Indexes))
  (for (_array_element _array_index) (Variables|Default|GetZombieSpawnPoints)
    (LocalVariables|SetL_ArrayIndex _array_index)
    (LocalVariables|SetL_PointDistance (Transformation|GetDistanceTo _array_element (Variables|Default|GetPriest)))
    (bind (_array_element_2 _array_index_2) (Utilities|Array|ForEachLoopwithBreak (LocalVariables|GetL_Distances) :!label _label)
      (:LoopBody
        (if (< (LocalVariables|GetL_PointDistance) _array_element_2)
          (Utilities|Array|Insert _l_distances (LocalVariables|GetL_PointDistance) _array_index_2)
          (Utilities|Array|RemoveIndex _l_distances 3)
          (Utilities|Array|Insert _l_indexes (LocalVariables|GetL_ArrayIndex) _array_index_2)
          (Utilities|Array|RemoveIndex _l_indexes 3)
          (goto _label Break)))))
  (return (LocalVariables|GetL_Indexes)))

(fn GetMinionsAmount
  (return (Utilities|Array|Length (Variables|Default|GetMinions))))

(fn GetMinions
  (return (Variables|Default|GetMinions)))

(fn GetZombieClass
  (LocalVariables|SetL_HealthCoefficient (Math|Float|Min(Float) (/ 0.1 (Class|ZombieBase|GetPercentHealth (Variables|Default|GetPriest))) 0.35))
  (if (Math|Random|RandomBoolwithWeight (+ 0.1 (LocalVariables|GetL_HealthCoefficient)))
    (return "/Game/BlueprintClasses/Zombies/ZombieClasses/BP_Zombie_Undying.BP_Zombie_Undying_C")
    (elif (Math|Random|RandomBoolwithWeight (+ 0.215 (LocalVariables|GetL_HealthCoefficient)))
      (return "/Game/BlueprintClasses/Zombies/ZombieClasses/BP_Zombie_Soldier.BP_Zombie_Soldier_C")
      (elif (Math|Random|RandomBoolwithWeight (+ 0.275 (LocalVariables|GetL_HealthCoefficient)))
        (return "/Game/BlueprintClasses/Zombies/ZombieClasses/BP_Zombie_Infected.BP_Zombie_Infected_C")
        (else
          (return "/Game/BlueprintClasses/Zombies/ZombieClasses/BP_Zombie_Turned.BP_Zombie_Turned_C"))))))

(fn CalculateBuffStrength
  (return (Math|Float|Min(Float) (/ 5.0 (Class|ZombieBase|GetPercentHealth (Variables|Default|GetPriest))) 12.5)))

(fn GetNextSkill
  (bind _skills_rownames (Variables|Default|GetSkills_RowNames))
  (bind (_outitem _outindex) (Utilities|Array|Random _skills_rownames))
  (for _array_element (Variables|Default|GetSkills_RowNames)
    (bind _returnvalue (Utilities|GetDataTableRow "/Game/Data/Gameplay/ST_PriestSkills.ST_PriestSkills" _array_element)
      (:then
        (if (Math|Random|RandomBoolwithWeight (.Priority (Utilities|Struct|BreakS_SkillInfo _returnvalue)))
          (bind _returnvalue_2 (Utilities|Time|SetTimerbyFunctionName self (.SkillName (Utilities|Struct|BreakS_SkillInfo _returnvalue)) 0.1))
          (Variables|Default|SetTH_CastedPerk _returnvalue_2)
          (return)))
      (:RowNotFound
        (Utilities|Array|RemoveItem (Variables|Default|GetSkills_RowNames) _array_element))))
  (bind _returnvalue_3 (Utilities|GetDataTableRow "/Game/Data/Gameplay/ST_PriestSkills.ST_PriestSkills" _outitem)
    (:then
      (bind _returnvalue_4 (Utilities|Time|SetTimerbyFunctionName self (Utilities|Struct|BreakS_SkillInfo _returnvalue_3) 0.1))
      (Variables|Default|SetTH_CastedPerk _returnvalue_4)
      (return))
    (:RowNotFound
      (Utilities|Array|RemoveIndex (Variables|Default|GetSkills_RowNames) _outindex)
      (Utilities|Time|SetTimerbyFunctionName 0 "UseAvailableSkill" 0.5))))

(fn RemoveUsedSkill
  (params (RowName :type Name))
  (Utilities|Array|RemoveItem (Variables|Default|GetSkills_RowNames) RowName)
  (bind _returnvalue (Utilities|GetDataTableRow "/Game/Data/Gameplay/ST_PriestSkills.ST_PriestSkills" RowName)
    (:then
      (return (Utilities|Struct|BreakS_SkillInfo _returnvalue)))
    (:RowNotFound
      (return 0.5))))

(fn AddSkillsBuffs
  (LocalVariables|SetL_TopBound (/ (Utilities|Array|Length (Variables|Default|GetSkills_RowNames)) 2))
  (for _array_element (Variables|Default|GetSkills_MinionBuffs)
    (Utilities|Array|Insert (Variables|Default|GetSkills_RowNames) _array_element (Math|Random|RandomIntegerinRange 0 (LocalVariables|GetL_TopBound))))
  (return))

(fn RemoveSkillsBuffs
  (for _array_element (Variables|Default|GetSkills_MinionBuffs)
    (Utilities|Array|RemoveItem (Variables|Default|GetSkills_RowNames) _array_element))
  (return))