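; AI controller for the Mutant zombie that chases the player, attacks when a move finishes and periodically leaps at them.
; Once StartLogic runs, a randomized timer, shorter during rage, schedules jump attacks, which require distance from the player and no rage cast.
; A looping timer also runs, and CheckJump can force an attempt when the last successful jump is too old.
; Both timers are cleared if MoveToPlayer finds the player invalid.
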(event Custom|StartLogic
  (CallFunction|MovetoPlayer)
  (bind _returnvalue (Utilities|Time|SetTimerbyEvent (EventDispatchers|CreateEvent :!event Custom|CheckJump) 3.0 true))
  (Variables|Default|SetTH_CheckJump _returnvalue))

(event Custom|MoveToPlayer
  (bind _player (Variables|Default|GetPlayer)
    (:then
      (if (not (Default|GetIsJumping (Variables|Default|GetMutant)))
        (AI|AIMoveTo self "0, 0, 0" _player 5e+01 "Default" "Default" true true
          (:then
            (if (not (Utilities|Time|IsTimerActivebyHandle (Variables|Default|GetTH_TimeForJump)))
              (bind _returnvalue (Utilities|Time|SetTimerbyEvent (EventDispatchers|CreateEvent :!event Custom|TimeForJumping) (CallFunction|GetJumpTime)))
              (Variables|Default|SetTH_TimeForJump _returnvalue)))
          (:OnMoveFinished
            (Default|Attack (Variables|Default|GetMutant) (Variables|Default|GetPlayer))))
        (else
          (Utilities|FlowControl|Delay 0.5)
          (CallFunction|MovetoPlayer))))
    (:else
      (CallFunction|StopTimers))))

(event Custom|TimeForJumping
  (Variables|Default|GetPlayer
    (:then
      (if (and (>= (Transformation|GetDistanceTo (Variables|Default|GetPlayer) (Variables|Default|GetMutant)) 5e+02) (not (Default|GetIsRageCasting (Variables|Default|GetMutant))))
        (Default|UseJumpAttack (Variables|Default|GetMutant))
        (Variables|Default|SetSuccessJump (Utilities|Time|GetTimeSeconds))))
    (:else)))

(event Custom|CheckJump
  (if (>= (- (Utilities|Time|GetTimeSeconds) (Variables|Default|GetSuccessJump)) 15.0)
    (if (not (Default|GetIsJumping (Variables|Default|GetMutant)))
      (Utilities|Time|PauseTimerbyHandle (Variables|Default|GetTH_TimeForJump))
      (CallFunction|TimeforJumping)
      (Utilities|FlowControl|Delay 2.0)
      (Utilities|Time|UnpauseTimerbyHandle (Variables|Default|GetTH_TimeForJump)))))

(event Custom|StopTimers
  (Utilities|Time|ClearandInvalidateTimerbyHandle (Variables|Default|GetTH_TimeForJump))
  (Utilities|Time|ClearandInvalidateTimerbyHandle (Variables|Default|GetTH_CheckJump)))

(event EventBeginPlay
  (Utilities|FlowControl|Delay 1.0)
  (bind _asbp_mutant (Utilities|Casting|CastToBP_Mutant (Pawn|GetControlledPawn)))
  (Variables|Default|SetMutant _asbp_mutant)
  (bind _asbp_nazi_zombie_character (Utilities|Casting|CastToBP_NaziZombieCharacter (Game|GetPlayerCharacter 0)))
  (Variables|Default|SetPlayer _asbp_nazi_zombie_character))

(fn ConstructionScript)

(fn GetJumpTime
  (if (Default|GetIsRage (Variables|Default|GetMutant))
    (return (Math|Random|RandomFloatinRange 5.0 1e+01))
    (else
      (return (Math|Random|RandomFloatinRange 8.0 15.0)))))