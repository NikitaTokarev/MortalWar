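; AI controller for zombies that chases a living player and triggers attacks, with setup run on authority.
; Online, a looping timer drives retargeting to the nearest living player character; offline, it targets player 0.
; AI MoveTo retries on failure and, on arrival, checks whether the zombie can attack before calling MultiPrepareAttack.
; AttackFinished resumes the chase, unpausing the retarget timer that is paused during online attacks.
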(event Custom|MoveToPlayer
  (AI|AIMoveTo (Pawn|GetControlledPawn) "0, 0, 0" (Variables|Default|GetClosestPlayer) 4e+01 true
    (:OnSuccess
      (bind (_dead _returnvalue) (Class|BPIEnemyBase|CanAttack(Message) (Pawn|GetControlledPawn)))
      (if (not _dead)
        (if _returnvalue
          (if (Variables|Default|GetbIsOnline)
            (Utilities|Time|PauseTimerbyHandle (Variables|Default|GetTH_FindClosestTarget)))
          (Default|MultiPrepareAttack (Variables|Default|GetControlledZombie) (Variables|Default|GetClosestPlayer)))))
    (:OnFail
      (bind _closestplayer (Variables|Default|GetClosestPlayer)
        (:then
          (if (not (Class|NaziZombieCharacter|GetIsDead _closestplayer))
            (CallFunction|MovetoPlayer)))
        (:else)))))

(event Custom|FindClosestEnemy
  (if (Variables|Default|GetbIsOnline)
    (Variables|Default|SetClosestPlayer 0)
    (Variables|Default|SetBestDistance 99999.0)
    (bind _outactors (Actor|GetAllActorsOfClass "/Game/BlueprintClasses/Player/BP_NaziZombieCharacter.BP_NaziZombieCharacter_C"))
    (for _array_element _outactors
      (if (not (Class|NaziZombieCharacter|GetIsDead _array_element))
        (if (< (Transformation|GetDistanceTo _array_element) (Variables|Default|GetBestDistance))
          (Variables|Default|SetClosestPlayer _array_element)
          (Variables|Default|SetBestDistance (Transformation|GetDistanceTo _array_element))))))
  (Utilities|IsValid (Variables|Default|GetClosestPlayer)
    (:Is%20Valid
      (if (not (Class|NaziZombieCharacter|GetIsDead (Variables|Default|GetClosestPlayer)))
        (CallFunction|MovetoPlayer)))))

(event EventBeginPlay
  (Networking|SwitchHasAuthority
    (:Authority
      (Utilities|FlowControl|Delay 0.25)
      (bind _asbp_zombie_base (Utilities|Casting|CastToBP_ZombieBase (Pawn|GetControlledPawn)))
      (Variables|Default|SetControlledZombie _asbp_zombie_base)
      (if (Class|BlueprintFunctionLibraryMisc|IsOnline self)
        (Variables|Default|SetbIsOnline true)
        (bind _returnvalue (Utilities|Time|SetTimerbyEvent (EventDispatchers|CreateEvent :!event Custom|FindClosestEnemy) 2.0 true))
        (Variables|Default|SetTH_FindClosestTarget _returnvalue)
        (else
          (bind _returnvalue_2 (Class|BPIPlayerCharacter|GetPlayerRef(Message) (Game|GetPlayerCharacter 0)))
          (Variables|Default|SetClosestPlayer _returnvalue_2)))
      (CallFunction|FindClosestEnemy))))

(event EventAttackFinished
  (if (Variables|Default|GetbIsOnline)
    (Utilities|Time|UnpauseTimerbyHandle (Variables|Default|GetTH_FindClosestTarget))
    (CallFunction|FindClosestEnemy)
    (elif (not (Class|NaziZombieCharacter|GetIsDead (Variables|Default|GetClosestPlayer)))
      (CallFunction|MovetoPlayer))))

(fn ConstructionScript)