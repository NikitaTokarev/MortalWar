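; BP_Area_DamnLand is a damage area, filed under zombie skills, that hurts the player while they stand inside it.
; When the player enters its Box, it applies damage at once and starts a looping half-second timer, stored by handle, for repeat hits.
; Leaving the Box clears and invalidates that timer, and other overlapping actors are ignored.
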(event OnComponentBeginOverlap(Box)
  (params (OverlappedComponent :type Primitive%20Component%20Object%20Reference) (OtherActor :type Actor%20Object%20Reference) (OtherComp :type Primitive%20Component%20Object%20Reference) (OtherBodyIndex :type Integer) (bFromSweep :type Boolean) (SweepResult :type Hit%20Result%20Structure%20%28by%20ref%29))
  (if (== OtherActor (CallFunction|GetPlayerChar))
    (CallFunction|AttackPlayer)
    (bind _returnvalue (Utilities|Time|SetTimerbyEvent (EventDispatchers|CreateEvent :!event Custom|AttackPlayer) 0.5 true))
    (Variables|Default|SetTH_AttackPlayer _returnvalue)))

(event OnComponentEndOverlap(Box)
  (params (OverlappedComponent :type Primitive%20Component%20Object%20Reference) (OtherActor :type Actor%20Object%20Reference) (OtherComp :type Primitive%20Component%20Object%20Reference) (OtherBodyIndex :type Integer))
  (if (== OtherActor (CallFunction|GetPlayerChar))
    (Utilities|Time|ClearandInvalidateTimerbyHandle (Variables|Default|GetTH_AttackPlayer))))

(event Custom|AttackPlayer
  (Game|Damage|ApplyDamage (CallFunction|GetPlayerChar) 1e+01 0 0))

(event EventBeginPlay
  (|CallParentFunction) ; This node is disabled and will not be called.\nDrag off pins to build functionality.
)

(event Collision|EventActorBeginOverlap
  (params (OtherActor :type Actor%20Object%20Reference))
  (|CallParentFunction OtherActor) ; This node is disabled and will not be called.\nDrag off pins to build functionality.
)

(event EventTick
  (params (DeltaSeconds :type Float%20%28single-precision%29))
  (|CallParentFunction DeltaSeconds) ; This node is disabled and will not be called.\nDrag off pins to build functionality.
)

(fn ConstructionScript
  (|CallParentFunction))