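; Aura of Power zombie skill actor that buffs zombies and feeds rage to BP_NaziZombieCharacter within its sphere, playing a Priest wave sound on BeginPlay.
; Sphere overlaps, ignoring the owner, toggle the aura buff on each BP_ZombieBase as it enters or leaves.
; For BP_NaziZombieCharacter, overlap starts a looping timer that increments rage until exit, using one stored character reference and timer handle.
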(event OnComponentBeginOverlap(Sphere)
  (params (OverlappedComponent :type Primitive%20Component%20Object%20Reference) (OtherActor :type Actor%20Object%20Reference) (OtherComp :type Primitive%20Component%20Object%20Reference) (OtherBodyIndex :type Integer) (bFromSweep :type Boolean) (SweepResult :type Hit%20Result%20Structure%20%28by%20ref%29))
  (if (!= OtherActor (Components|GetOwner))
    (bind _asbp_zombie_base (Utilities|Casting|CastToBP_ZombieBase OtherActor)
      (:then
        (Default|ActivateBuffAuraOfPower _asbp_zombie_base))
      (:CastFailed
        (bind _asbp_nazi_zombie_character (Utilities|Casting|CastToBP_NaziZombieCharacter OtherActor))
        (bind _returnvalue (Utilities|Time|SetTimerbyEvent (delegate Custom|RecoveryRage) 0.3 true))
        (Variables|Default|SetTH_RecoveryRage _returnvalue)))))

(event OnComponentEndOverlap(Sphere)
  (params (OverlappedComponent :type Primitive%20Component%20Object%20Reference) (OtherActor :type Actor%20Object%20Reference) (OtherComp :type Primitive%20Component%20Object%20Reference) (OtherBodyIndex :type Integer))
  (if (!= OtherActor (Components|GetOwner))
    (bind _asbp_zombie_base (Utilities|Casting|CastToBP_ZombieBase OtherActor)
      (:then
        (Default|DectivateBuffAuraOfPower _asbp_zombie_base))
      (:CastFailed
        (Utilities|Casting|CastToBP_NaziZombieCharacter OtherActor)
        (Utilities|Time|ClearandInvalidateTimerbyHandle (Variables|Default|GetTH_RecoveryRage))))))

(event Custom|RecoveryRage
  (Class|NaziZombieCharacter|IncrementRage (stale OnComponentBeginOverlap(Sphere) _asbp_nazi_zombie_character) 1.5))

(event EventBeginPlay
  (Audio|PlaySoundatLocation "/Game/Audio/Characters/Bosses/Priest/S_Priest_AuraOfPower_Wave.S_Priest_AuraOfPower_Wave" (Transformation|GetActorLocation) "0, 0, 0" 1.0 1.0 0.0 0 0 0))

(fn ConstructionScript)