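; BP_Projectile_Curse is a zombie skill projectile that temporarily curses the character it targets.
; BeginPlay caches the parent's target actor as a BP_NaziZombieCharacter.
; On overlap it hides itself, clears its lifespan and applies the curse to that cached target, removing it after a nine-second delay if still active.
; If the curse fails to apply, a short lifespan destroys the projectile instead.
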(event EventOnOverlap
  (Actor|SetLifeSpan 0.0)
  (Rendering|SetActorHiddenInGame true)
  (bind _returnvalue (Default|AddCurse (Variables|Default|GetTargetPlayer) "NewEnumerator0"))
  (if _returnvalue
    (Utilities|FlowControl|Delay 9.0)
    (if (Default|GetIsCursed (Variables|Default|GetTargetPlayer))
      (Default|RemoveCurse (Variables|Default|GetTargetPlayer) "NewEnumerator0"))
    (else
      (Actor|SetLifeSpan 0.2))))

(event EventBeginPlay
  (|CallParentFunction)
  (bind _asbp_nazi_zombie_character (Utilities|Casting|CastToBP_NaziZombieCharacter (CallFunction|GetTargetActor)))
  (Variables|Default|SetTargetPlayer _asbp_nazi_zombie_character))

(event EventTick
  (params (DeltaSeconds :type Float%20%28single-precision%29))
  (|CallParentFunction DeltaSeconds))

(fn ConstructionScript
  (|CallParentFunction))