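; Base homing projectile for zombie skills, with an empty OnOverlap event as the impact hook.
; Every Tick it eases toward a point 75 units above Target, stepping proportionally to remaining distance and yawing to face it.
; Overlapping a BP_NaziZombieCharacter fires OnOverlap, then disables capsule collision.
; BeginPlay records the start location and sets IsMoving after a short delay, but movement does not check that flag.
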(event OnComponentBeginOverlap(Capsule)
  (params (OverlappedComponent :type Primitive%20Component%20Object%20Reference) (OtherActor :type Actor%20Object%20Reference) (OtherComp :type Primitive%20Component%20Object%20Reference) (OtherBodyIndex :type Integer) (bFromSweep :type Boolean) (SweepResult :type Hit%20Result%20Structure%20%28by%20ref%29))
  (Utilities|Casting|CastToBP_NaziZombieCharacter OtherActor)
  (CallFunction|OnOverlap)
  (Collision|SetCollisionEnabled (Variables|Default|GetCapsule) "NoCollision"))

(event Custom|OnOverlap)

(event EventTick
  (params (DeltaSeconds :type Float%20%28single-precision%29))
  (bind (_location _rotation) (CallFunction|VInterptoMine))
  (Transformation|SetActorLocationAndRotation _location (Math|Rotator|MakeRotator 0.0 0.0 (.yaw _rotation))))

(event EventBeginPlay
  (Variables|Default|SetStartLocation (Transformation|GetActorLocation))
  (Variables|Default|GetTarget
    (:then
      (Utilities|FlowControl|Delay 0.1)
      (Variables|Default|SetbIsMoving true))
    (:else)))

(fn ConstructionScript)

(fn GetTargetActor
  (return (Variables|Default|GetTarget)))

(fn VInterptoMine
  (LocalVariables|SetL_Dist (- (+ (Transformation|GetActorLocation (Variables|Default|GetTarget)) "0, 0,75.000000") (Transformation|GetActorLocation)))
  (LocalVariables|SetL_DeltaMove (* (LocalVariables|GetL_Dist) (* (Variables|Default|GetSpeed) (Utilities|Time|GetWorldDeltaSeconds))))
  (return (+ (Transformation|GetActorLocation) (LocalVariables|GetL_DeltaMove)) (Math|Rotator|FindLookatRotation (Transformation|GetActorLocation) (Transformation|GetActorLocation (Variables|Default|GetTarget)))))