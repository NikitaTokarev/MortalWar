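; BP_Projectile_LifeSphere is a healing projectile from the zombie skill set that restores health to whatever it touches.
; On capsule overlap it hides itself, then casts the other actor to decide the effect.
; Zombies gain health through ChangeHealth, with BP_Priest receiving a larger amount than other zombies.
; BP_NaziZombieCharacter instead recovers a small amount of health and has its negative effects disabled.
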(event OnComponentBeginOverlap(Capsule)
  (params (OverlappedComponent :type Primitive%20Component%20Object%20Reference) (OtherActor :type Actor%20Object%20Reference) (OtherComp :type Primitive%20Component%20Object%20Reference) (OtherBodyIndex :type Integer) (bFromSweep :type Boolean) (SweepResult :type Hit%20Result%20Structure%20%28by%20ref%29))
  (Rendering|SetActorHiddenInGame true)
  (bind _asbp_zombie_base (Utilities|Casting|CastToBP_ZombieBase OtherActor)
    (:then
      (bind _asbp_priest (Utilities|Casting|CastToBP_Priest _asbp_zombie_base)
        (:then
          (Class|ZombieBase|ChangeHealth _asbp_priest 675.0))
        (:CastFailed
          (Class|ZombieBase|ChangeHealth _asbp_zombie_base 3.5e+02))))
    (:CastFailed
      (bind _asbp_nazi_zombie_character (Utilities|Casting|CastToBP_NaziZombieCharacter OtherActor))
      (Class|NaziZombieCharacter|RecoveryHealth _asbp_nazi_zombie_character 15.0)
      (Default|DisableNegativeEffects _asbp_nazi_zombie_character))))

(event EventBeginPlay
  (|CallParentFunction))

(event EventTick
  (params (DeltaSeconds :type Float%20%28single-precision%29))
  (|CallParentFunction DeltaSeconds))

(fn ConstructionScript
  (|CallParentFunction))