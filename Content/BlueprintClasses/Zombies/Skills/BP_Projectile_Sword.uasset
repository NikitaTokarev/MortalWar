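; Sword projectile for a zombie skill that damages its target player character and may inflict a temporary curse.
; BeginPlay caches the target; overlap hides the projectile and damages that cached character.
; Unless the target is effect-immune, cascading weighted rolls attempt one of three curses.
; The hidden actor clears its lifespan to stay alive through the random curse duration, removes the curse, then expires shortly after.
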(event EventBeginPlay
  (|CallParentFunction)
  (bind _asbp_nazi_zombie_character (Utilities|Casting|CastToBP_NaziZombieCharacter (CallFunction|GetTargetActor)))
  (Variables|Default|SetPlayerChar _asbp_nazi_zombie_character))

(event EventOnOverlap
  (bind _playerchar (Variables|Default|GetPlayerChar))
  (Actor|SetLifeSpan 0.0)
  (Rendering|SetActorHiddenInGame true)
  (Game|Damage|ApplyDamage _playerchar 25.0 0 0)
  (if (not (Default|GetIsImmunetoEffects _playerchar))
    (if (Math|Random|RandomBoolwithWeight 0.2)
      (bind _returnvalue (Default|AddCurse (Variables|Default|GetPlayerChar) "NewEnumerator1"))
      (if _returnvalue
        (Utilities|FlowControl|Delay (Math|Random|RandomFloatinRange 7.0 1e+01))
        (Default|RemoveCurse (Variables|Default|GetPlayerChar) "NewEnumerator1")
        (Actor|SetLifeSpan 0.2)
        (else
          (Actor|SetLifeSpan 0.2)))
      (elif (Math|Random|RandomBoolwithWeight 0.2)
        (bind _returnvalue_2 (Default|AddCurse (Variables|Default|GetPlayerChar) "NewEnumerator2"))
        (if _returnvalue_2
          (Utilities|FlowControl|Delay (Math|Random|RandomFloatinRange 7.0 1e+01))
          (Default|RemoveCurse (Variables|Default|GetPlayerChar) "NewEnumerator2")
          (Actor|SetLifeSpan 0.2)
          (else
            (Actor|SetLifeSpan 0.2)))
        (elif (Math|Random|RandomBoolwithWeight 0.075)
          (bind _returnvalue_3 (Default|AddCurse (Variables|Default|GetPlayerChar) "NewEnumerator0"))
          (if _returnvalue_3
            (Utilities|FlowControl|Delay (Math|Random|RandomFloatinRange 6.0 8.0))
            (Default|RemoveCurse (Variables|Default|GetPlayerChar) "NewEnumerator0")
            (Actor|SetLifeSpan 0.2)
            (else
              (Actor|SetLifeSpan 0.2)))
          (else
            (Actor|SetLifeSpan 0.2)))))
    (else
      (Actor|SetLifeSpan 0.2))))

(fn ConstructionScript
  (|CallParentFunction))