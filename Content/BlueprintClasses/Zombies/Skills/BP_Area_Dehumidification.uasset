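; BP_Area_Dehumidification is a zombie skill area, owned by a BP_Priest, that drains the player's health to feed the Priest.
; Player overlap with its Box triggers an immediate attack, starts a looping half-second timer and activates audio.
; Each attack damages the player and calls ChangeHealth on the cached Priest with a larger positive amount.
; Leaving the Box clears the timer and stops the audio.
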(event OnComponentBeginOverlap(Box)
  (params (OverlappedComponent :type Primitive%20Component%20Object%20Reference) (OtherActor :type Actor%20Object%20Reference) (OtherComp :type Primitive%20Component%20Object%20Reference) (OtherBodyIndex :type Integer) (bFromSweep :type Boolean) (SweepResult :type Hit%20Result%20Structure%20%28by%20ref%29))
  (if (== OtherActor (CallFunction|GetPlayerChar))
    (CallFunction|AttackPlayer)
    (bind _returnvalue (Utilities|Time|SetTimerbyEvent (EventDispatchers|CreateEvent :!event Custom|AttackPlayer) 0.5 true))
    (Variables|Default|SetTH_AttackPlayer _returnvalue)
    (Components|Activation|Activate (Variables|Default|GetAudio) false)))

(event OnComponentEndOverlap(Box)
  (params (OverlappedComponent :type Primitive%20Component%20Object%20Reference) (OtherActor :type Actor%20Object%20Reference) (OtherComp :type Primitive%20Component%20Object%20Reference) (OtherBodyIndex :type Integer))
  (if (== OtherActor (CallFunction|GetPlayerChar))
    (Utilities|Time|ClearandInvalidateTimerbyHandle (Variables|Default|GetTH_AttackPlayer))
    (Audio|Components|Audio|Stop (Variables|Default|GetAudio))))

(event Custom|AttackPlayer
  (Game|Damage|ApplyDamage (CallFunction|GetPlayerChar) 6.0 0 0)
  (Class|ZombieBase|ChangeHealth (Variables|Default|GetPriest) 3e+01))

(event EventBeginPlay
  (|CallParentFunction)
  (bind _asbp_priest (Utilities|Casting|CastToBP_Priest (Components|GetOwner)))
  (Variables|Default|SetPriest _asbp_priest))

(fn ConstructionScript
  (|CallParentFunction))