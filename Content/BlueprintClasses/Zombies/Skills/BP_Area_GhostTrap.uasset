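; BP_Area_GhostTrap is a zombie skill area that acts as a trap, stunning the player who steps into it.
; Overlapping its Box with the player applies the stun, switches the particle system to the active ghost trap effect and sets a fallback lifespan.
; A timer started on overlap, presumably bound to RestunPlayer, clears the stun after a few seconds and shortens the lifespan so the trap disappears.
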(event OnComponentBeginOverlap(Box)
  (params (OverlappedComponent :type Primitive%20Component%20Object%20Reference) (OtherActor :type Actor%20Object%20Reference) (OtherComp :type Primitive%20Component%20Object%20Reference) (OtherBodyIndex :type Integer) (bFromSweep :type Boolean) (SweepResult :type Hit%20Result%20Structure%20%28by%20ref%29))
  (bind _returnvalue (CallFunction|GetPlayerChar))
  (if (== OtherActor _returnvalue)
    (Class|CharacterBase|SetPlayerIsStun _returnvalue true)
    (Actor|SetLifeSpan 1e+01)
    (Effects|Components|ParticleSystem|SetTemplate (Variables|Default|GetParticleSystem) "/Game/Assets/InfinityBladeEffects/Effects/FX_Archive/P_GhostTrap_Active.P_GhostTrap_Active")
    (bind _returnvalue_2 (Utilities|Time|SetTimerbyEvent (EventDispatchers|CreateEvent :!event Custom|RestunPlayer) 3.5))
    (Variables|Default|SetTH_ResetStun _returnvalue_2)))

(event Custom|RestunPlayer
  (bind _returnvalue (CallFunction|GetPlayerChar))
  (if (Variables|/Script/WorldAtWar.CharacterBase|GetbIsStunned _returnvalue)
    (Class|CharacterBase|SetPlayerIsStun _returnvalue false))
  (Actor|SetLifeSpan 0.1))

(event EventBeginPlay
  (|CallParentFunction))

(fn ConstructionScript
  (|CallParentFunction))