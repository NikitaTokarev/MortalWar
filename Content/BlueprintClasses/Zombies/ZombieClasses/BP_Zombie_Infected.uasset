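; BP_Zombie_Infected is a zombie variant that can infect players with a timed, damaging disease.
; On BeginPlay it binds Disease to its successful-attack event, which rolls InfectedChance against players not already infected and calls ServerImposeDisease on a hit.
; ChangeEffectChance scales that chance by a multiplier, and GetChestBone supplies this zombie's ribcage bone name.
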(event Custom|Disease
  (params (Player :type BP%20Nazi%20Zombie%20Character%20Object%20Reference))
  (if (not (Variables|/Script/WorldAtWar.NaziZombieCharacter|GetbIsInfected Player))
    (if (Math|Random|RandomBoolwithWeight (Variables|ZombieBase|GetInfectedChance))
      (Class|NaziZombieCharacter|ServerImposeDisease Player 1e+01 3.0))))

(event EventBeginPlay
  (|CallParentFunction)
  (EventDispatchers|BindEventtoOnAttackSuccessfully (delegate Custom|Disease)))

(event EventChangeEffectChance
  (params (Multiplier :type Float%20%28single-precision%29))
  (Variables|ZombieBase|SetInfectedChance (* Multiplier (Variables|ZombieBase|GetInfectedChance))))

(fn ConstructionScript
  (|CallParentFunction))

(fn GetChestBone
  (return (Utilities|Name|MakeLiteralName "Base-HumanRibcage")))