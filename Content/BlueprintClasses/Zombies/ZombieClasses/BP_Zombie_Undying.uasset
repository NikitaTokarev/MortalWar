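; Undying zombie variant that, on its first death, has a weighted chance to resurrect as a crawler instead of dying.
; Resurrection plays a death montage, briefly hides the actor, swaps in the crawl attack and restores movement, with authority handling the resurrect, forward offset and AI retargeting.
; A failed roll or DestroyCharacter plays a long death before parent Die.
; State flags block attacks while resurrecting or dying, and speed buffs once resurrection begins.
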(event Custom|Multi_Resurrection
  (bind _returnvalue (Transformation|GetActorForwardVector))
  (bind _attackmontages (Variables|Default|GetAttackMontages))
  (Audio|Components|Audio|Stop (Variables|Default|GetS_Zombie_Roar_Cue))
  (Variables|/Script/Engine.CharacterMovementComponent|SetRotationRate (Variables|Character|GetCharacterMovement) "0, 0, 0")
  (Variables|Default|SetbPrepareToResurrect true)
  (Collision|SetCollisionResponsetoChannel (Variables|Character|GetMesh) "ECC_GameTraceChannel2" "ECR_Ignore")
  (Collision|SetCollisionResponsetoChannel (Variables|Default|GetCapsuleComponent) "ECC_Pawn" "ECR_Ignore")
  (Variables|/Script/Engine.CharacterMovementComponent|SetMaxWalkSpeed (Variables|Character|GetCharacterMovement) 0.0)
  (bind _returnvalue_2 (Animation|PlayAnimMontage "/Game/BlueprintClasses/Zombies/Animations/Zombie_Undying/AM_Zombie_Undying_Death.AM_Zombie_Undying_Death" 1.0 "None"))
  (Utilities|FlowControl|Delay (- _returnvalue_2 0.5))
  (Collision|SetCollisionResponsetoChannel (Variables|Default|GetCapsuleComponent) "ECC_Pawn" "ECR_Block")
  (Networking|SwitchHasAuthority
    (:Authority
      (Utilities|FlowControl|Delay 0.5)
      (Class|ZombieBase|Resurrect)
      (Transformation|AddActorWorldOffset (Math|Vector|MakeVector (* (.x _returnvalue) 1e+02) (* (.y _returnvalue) 1e+02) 0.0)))
    (:Remote
      _))
  (Rendering|SetActorHiddenInGame true)
  (Variables|Default|SetbIsResurrected true)
  (Default|CallOnResurrecting)
  (Audio|PlaySoundatLocation "/Game/Audio/Characters/Zombies/Resurrected/S_Zombie_Resurrected_Resurrect.S_Zombie_Resurrected_Resurrect" (Transformation|GetActorLocation) "0, 0, 0" 1.0 1.0 0.0 "/Game/Audio/Settings/SA_CharacterEffects.SA_CharacterEffects" 0 0)
  (Utilities|FlowControl|Delay 0.05)
  (Rendering|SetActorHiddenInGame false)
  (Utilities|FlowControl|Delay 0.45)
  (Collision|SetCollisionResponsetoChannel (Variables|Character|GetMesh) "ECC_GameTraceChannel2" "ECR_Block")
  (Utilities|FlowControl|Delay 1.3)
  (Variables|/Script/Engine.CharacterMovementComponent|SetMaxWalkSpeed (Variables|Character|GetCharacterMovement) 1.4e+02)
  (Utilities|Array|Clear _attackmontages)
  (Utilities|Array|Add _attackmontages "/Game/BlueprintClasses/Zombies/Animations/Zombie_Undying/AM_Zombie_Undying_Crawl_Attack.AM_Zombie_Undying_Crawl_Attack")
  (Variables|Default|SetbPrepareToResurrect false)
  (Variables|/Script/Engine.CharacterMovementComponent|SetRotationRate (Variables|Character|GetCharacterMovement) "0,290.000000, 0")
  (Audio|Components|Audio|Play (Variables|Default|GetS_Zombie_Roar_Cue) 0.0)
  (Networking|SwitchHasAuthority
    (:Authority
      (bind _asbp_aicontroller_zombie (Utilities|Casting|CastToBP_AIController_Zombie (Pawn|GetController)))
      (Default|FindClosestEnemy _asbp_aicontroller_zombie))))

(event Custom|Multi_Death
  (Audio|Components|Audio|Stop (Variables|Default|GetS_Zombie_Roar_Cue))
  (Variables|Default|SetbThisEnd true)
  (Variables|Default|SetbPrepareToResurrect false)
  (Variables|/Script/Engine.CharacterMovementComponent|SetMaxWalkSpeed (Variables|Character|GetCharacterMovement) 0.0)
  (Collision|SetCollisionResponsetoChannel (Variables|Character|GetMesh) "ECC_GameTraceChannel2" "ECR_Ignore")
  (Animation|PlayAnimMontage "/Game/BlueprintClasses/Zombies/Animations/Zombie_Undying/AM_Zombie_Undying_Death_Long.AM_Zombie_Undying_Death_Long" 1.0 "None")
  (Utilities|FlowControl|Delay 2e+01)
  (Rendering|SetActorHiddenInGame true))

(event EventBeginPlay
  (|CallParentFunction) ; This node is disabled and will not be called.\nDrag off pins to build functionality.
)

(event EventDestroyCharacter
  (CallFunction|MultiDeath)
  (Utilities|FlowControl|Delay 1.0)
  (|CallParentFunction))

(event EventDie
  (if (Variables|Default|GetbIsResurrected)
    (Variables|Default|SetbPrepareToResurrect true)
    (Variables|Default|SetbThisEnd true)
    (Audio|Components|Audio|Stop (Variables|Default|GetS_Zombie_Roar_Cue))
    (|CallParentFunction)
    (elif (Math|Random|RandomBoolwithWeight (Variables|ZombieBase|GetRessurectChance))
      (CallFunction|MultiResurrection)
      (else
        (CallFunction|MultiDeath)
        (Utilities|FlowControl|Delay 1.0)
        (|CallParentFunction)))))

(fn ConstructionScript
  (|CallParentFunction))

(fn CanAttack
  (return (Variables|Default|GetbIsDead) (Math|Boolean|ANDBoolean (not (Variables|Default|GetbIsDead)) (not (Variables|Default|GetbPrepareToResurrect)) (not (Variables|Default|GetbThisEnd)))))

(fn CanActivateSpeedBuff
  (return (and (not (Variables|Default|GetbIsResurrected)) (not (Variables|Default|GetbPrepareToResurrect)))))

(fn GetChestBone
  (return "s_BuffPlace"))