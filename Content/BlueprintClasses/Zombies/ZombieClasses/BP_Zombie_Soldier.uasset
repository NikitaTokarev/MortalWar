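; Soldier zombie Blueprint that can fly into a temporary rage when it takes damage.
; On the server, each hit rolls RageChance to double its damage and raise walk speed through Multi_ChangeMaxSpeed, accounting for any speed buff.
; A timer later halves damage and lowers speed, then a short delay gates the next rage.
; It also supports rage-chance scaling, a buff body tint and Neck as the chest bone.
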(event Custom|OnTakeAnyDamage_Event_0
  (params (DamagedActor :type Actor%20Object%20Reference) (Damage :type Float%20%28single-precision%29) (DamageType :type Damage%20Type%20Object%20Reference) (InstigatedBy :type Controller%20Object%20Reference) (DamageCauser :type Actor%20Object%20Reference))
  (if (not (Variables|Default|GetbIsAnger))
    (if (Math|Random|RandomBoolwithWeight (Variables|Default|GetRageChance))
      (Variables|Default|SetbIsAnger true)
      (Variables|Default|SetDamage (* (Class|ZombieBase|GetDamage) 2.0))
      (CallFunction|MultiChangeMaxSpeed (select (CallFunction|IsSpeedBuff) 3.8e+02 3.5e+02))
      (Utilities|Time|SetTimerbyEvent (delegate Custom|AngerFinished) 15.0))))

(event Custom|Multi_ChangeMaxSpeed
  (params (MaxSpeed :type Float%20%28single-precision%29))
  (Variables|/Script/Engine.CharacterMovementComponent|SetMaxWalkSpeed (Variables|Character|GetCharacterMovement) MaxSpeed))

(event Custom|AngerFinished
  (Variables|Default|SetDamage (* (Class|ZombieBase|GetDamage) 0.5))
  (CallFunction|MultiChangeMaxSpeed (select (CallFunction|IsSpeedBuff) 225.0 1.5e+02))
  (Utilities|FlowControl|Delay 7.0)
  (Variables|Default|SetbIsAnger false))

(event EventBeginPlay
  (|CallParentFunction)
  (Networking|SwitchHasAuthority
    (:Authority
      (EventDispatchers|AssignOnTakeAnyDamage (delegate Custom|OnTakeAnyDamage_Event_0)))))

(event EventPlayBuffVFX
  (bind _mesh (Variables|Character|GetMesh))
  (bind _returnvalue (Rendering|Material|CreateDynamicMaterialInstance _mesh 0 (Rendering|Material|GetMaterial _mesh 0) "None" :!class /Script/Engine.PrimitiveComponent))
  (Rendering|Material|SetVectorParameterValue _returnvalue "BodyColor" "(R=1.000000,G=0.654167,B=0.658961,A=1.000000)" :!class /Script/Engine.MaterialInstanceDynamic))

(event EventChangeEffectChance
  (params (Multiplier :type Float%20%28single-precision%29))
  (Variables|Default|SetRageChance (* Multiplier (Variables|Default|GetRageChance))))

(fn ConstructionScript
  (|CallParentFunction))

(fn GetChestBone
  (return (Utilities|Name|MakeLiteralName "Neck")))