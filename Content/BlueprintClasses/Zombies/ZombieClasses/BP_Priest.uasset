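; BP_Priest is a boss zombie Blueprint that shares incoming damage with its minions.
; On begin play it caches its BP_AIController_Priest after a short delay, and boss activation has that controller use an available skill.
; While minions exist, damage is divided by their count and that share hits the priest and every minion; otherwise the priest takes it all.
; Helpers expose the anim instance and right-hand socket location.
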(event Custom|ActivateBoss
  (Utilities|FlowControl|Delay 0.5)
  (Default|UseAvailableSkill (Variables|Default|GetPriestController)))

(event EventBeginPlay
  (|CallParentFunction)
  (Utilities|FlowControl|Delay 1.0)
  (bind _asbp_aicontroller_priest (Utilities|Casting|CastToBP_AIController_Priest (Pawn|GetController)))
  (Variables|Default|SetPriestController _asbp_aicontroller_priest))

(event EventDecrementHealth
  (params (InDamage :type Integer))
  (CallFunction|TakeDamage InDamage))

(fn ConstructionScript
  (|CallParentFunction))

(fn GetAnimInstance
  (return (Components|SkeletalMesh|GetAnimInstance (Variables|Character|GetMesh))))

(fn TakeDamage
  (params (InDamage :type Integer))
  (bind _priestcontroller (Variables|Default|GetPriestController)
    (:then
      (if (> (Default|GetMinionsAmount _priestcontroller) 0)
        (bind _output_get (LocalVariables|SetL_Damage (/ InDamage (Default|GetMinionsAmount _priestcontroller))))
        (|CallParentFunction _output_get)
        (for _array_element (Default|GetMinions (Variables|Default|GetPriestController))
          (Class|ZombieBase|DecrementHealth _array_element (LocalVariables|GetL_Damage)))
        (return)
        (else
          _)))
    (:else
      _))
  (|CallParentFunction InDamage)
  (return))

(fn GetRightHandLocation
  (return (Transformation|GetSocketLocation (Variables|Character|GetMesh) "s_RightHand")))