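; Mutant boss zombie with punch and swipe attacks, a timer-interpolated leap that deals radial damage, and AI controller-driven movement.
; Taking damage can trigger a roaring rage that changes speed, resistances and attack strength and can chain jumps, with odds and duration scaling as health drops.
; Montage lengths pace actions, and notify events drive box-trace hits and sounds.
; During rage, ranged hits refill player rage and melee hits restore player health.
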(event Custom|ActivateBoss
  ;[1 0.9457 0] Activation
  (bind _asbp_aicontroller_mutant (Utilities|Casting|CastToBP_AIController_Mutant (Pawn|GetController)))
  (bind _output_get (Variables|Default|SetBP_Controller _asbp_aicontroller_mutant))
  (Default|StartLogic _output_get))

(event Custom|Attack
  (params (TargetPlayer :type BP%20Nazi%20Zombie%20Character%20Object%20Reference))
  ;[0.3302 0.3232 0.1392 1 32] Base Attacks
  (if (Math|Boolean|ANDBoolean (not (Variables|Default|GetbIsJumping)) (not (Variables|Default|GetbIsRageCasting)) (not (Variables|Default|GetbIsDead)))
    (Utilities|FlowControl|Delay 0.1)
    (CallFunction|RotatetoPlayer TargetPlayer)
    (bind _returnvalue (CallFunction|AttackPlayer TargetPlayer))
    (Utilities|FlowControl|Delay _returnvalue)
    (bind _bp_controller (Variables|Default|GetBP_Controller)
      (:then
        (Default|MovetoPlayer _bp_controller))
      (:else))))

(event Custom|UseJumpAttack
  ;[0.9379 0 1 1 32] Jump Attack
  (if (not (Variables|Default|GetbIsJumping))
    (CallFunction|RotatetoPlayer (Game|GetPlayerCharacter 0))
    (Variables|Default|SetbIsJumping true)
    (Variables|/Script/Engine.CharacterMovementComponent|SetMaxWalkSpeed (Variables|Character|GetCharacterMovement) 0.0)
    (bind _returnvalue (Animation|Montage|MontagePlay (Components|SkeletalMesh|GetAnimInstance (Variables|Character|GetMesh)) "/Game/BlueprintClasses/Zombies/Animations/Boss_Mutant/AM_Mutant_Jump_Attack.AM_Mutant_Jump_Attack" 1.0 "MontageLength" 0.0 true))
    (Utilities|FlowControl|Delay (- _returnvalue 0.5))
    (CallFunction|SetLocationAfterJump)
    (if (not (Variables|Default|GetbIsRage))
      (Utilities|FlowControl|Delay 0.02 :!label _label)
      (Variables|/Script/Engine.CharacterMovementComponent|SetMaxWalkSpeed (Variables|Character|GetCharacterMovement) (select (Variables|Default|GetbIsRageCasting) 0.0 (select (Variables|Default|GetbIsRage) 3.5e+02 2e+02)))
      (Variables|Default|SetbIsJumping false)
      (bind _bp_controller (Variables|Default|GetBP_Controller)
        (:then
          (Default|MovetoPlayer _bp_controller))
        (:else))
      (elif (not (CallFunction|ShouldJumpAgain))
        (goto _label)
        (else
          (Variables|Default|SetbIsJumping false)
          (CallFunction|UseJumpAttack))))))

(event Custom|JumpsControl
  ;[0.9379 0 1 1 32] Jump Attack
  (bind _returnvalue (Utilities|Time|SetTimerbyEvent (delegate Custom|Flying) 0.01 true))
  (Variables|Default|SetTH_Jump _returnvalue)
  (Variables|Default|SetTargetJumpLocation (Transformation|GetActorLocation (Game|GetPlayerCharacter 0))))

(event Custom|Flying
  ;[0.9379 0 1 1 32] Jump Attack
  (CallFunction|VInterptoMine)
  (bind _result (Math|Integer|IncrementInt (Variables|Default|GetJumpsIteration))
    (:%20%20
      (if (== _result 100)
        (Utilities|Time|ClearandInvalidateTimerbyHandle (Variables|Default|GetTH_Jump))
        (Variables|Default|SetJumpsIteration 0)))))

(event Custom|OnTakeDamage_Melee
  (params (Player :type Nazi%20Zombie%20Character%20Object%20Reference) (Damage :type Float%20%28single-precision%29))
  (if (Variables|Default|GetbIsRage)
    (Class|NaziZombieCharacter|RecoveryHealth Player (* (/ Damage (Variables|Default|GetMaxHealth)) 105.0))))

(event Custom|OnTakeDamage
  (params (DamagedActor :type Actor%20Object%20Reference) (Damage :type Float%20%28single-precision%29) (DamageType :type Damage%20Type%20Object%20Reference) (InstigatedBy :type Controller%20Object%20Reference) (DamageCauser :type Actor%20Object%20Reference))
  ;[1 0 0.01478 1 32] RAGE
  (if (and (not (Variables|Default|GetbIsDead)) (not (Variables|Default|GetbIsJumping)))
    (if (and (Variables|Default|GetbRageEnabled) (Math|Random|RandomBoolwithWeight (Math|Float|Min(Float) (/ 0.23 (Class|ZombieBase|GetPercentHealth)) 0.75)))
      (Variables|Default|SetbRageEnabled false)
      (Variables|Default|SetbIsRageCasting true)
      (Variables|/Script/Engine.CharacterMovementComponent|SetMaxWalkSpeed (Variables|Character|GetCharacterMovement) 0.0)
      (bind _returnvalue (Animation|Montage|MontagePlay (Components|SkeletalMesh|GetAnimInstance (Variables|Character|GetMesh)) "/Game/BlueprintClasses/Zombies/Animations/Boss_Mutant/AM_Mutant_Roaring.AM_Mutant_Roaring" 1.5 "MontageLength" 0.0 true))
      (Utilities|FlowControl|Delay (/ _returnvalue 1.5))
      (Variables|Default|SetbIsRage true)
      (Utilities|Time|SetTimerbyEvent (delegate Custom|DisableRage) (Math|Float|Clamp(Float) (/ 1e+01 (Class|ZombieBase|GetPercentHealth)) 10.5 25.0))
      (if (not (Variables|Default|GetbIsDead))
        (Variables|Default|SetbIsRageCasting false)
        (Utilities|Struct|SetmembersinResistanceData (Variables|Default|GetResistances) 1.0 2.0 0.6)
        (Variables|/Script/Engine.CharacterMovementComponent|SetMaxWalkSpeed (Variables|Character|GetCharacterMovement) 3.5e+02)
        (bind _bp_controller (Variables|Default|GetBP_Controller)
          (:then
            (Default|MovetoPlayer _bp_controller))
          (:else))))))

(event Custom|DisableRage
  ;[1 0 0.01478 1 32] RAGE
  (if (not (Variables|Default|GetbIsDead))
    (Variables|Default|SetbIsRage false)
    (Utilities|Struct|SetmembersinResistanceData (Variables|Default|GetResistances) 0.75 1.25 0.5)
    (if (not (Variables|Default|GetbIsJumping))
      (Variables|/Script/Engine.CharacterMovementComponent|SetMaxWalkSpeed (Variables|Character|GetCharacterMovement) 2e+02))
    (Utilities|FlowControl|Delay (* 12.0 (Class|ZombieBase|GetPercentHealth)))
    (Variables|Default|SetbRageEnabled true)))

(event Custom|OnDeathEvent
  (params (Enemy :type Zombie%20Base%20Object%20Reference))
  (bind _mesh (Variables|Character|GetMesh))
  (bind _bp_controller (Variables|Default|GetBP_Controller))
  (bind _returnvalue (Components|SkeletalMesh|GetAnimInstance _mesh))
  (bind _returnvalue_2 (Animation|Montage|GetCurrentActiveMontage _returnvalue))
  ;[0 0 0] DEATH
  (Utilities|Time|ClearandInvalidateTimerbyHandle (Variables|Default|GetTH_Jump))
  (Variables|/Script/Engine.CharacterMovementComponent|SetMaxWalkSpeed (Variables|Character|GetCharacterMovement) 0.0)
  (AI|Navigation|StopMovement _bp_controller)
  (Default|StopTimers _bp_controller)
  (Actor|DestroyActor _bp_controller)
  (Utilities|IsValid _returnvalue_2
    (:Is%20Valid
      (Animation|Montage|MontageStop _returnvalue 0.0 _returnvalue_2))))

(event Custom|OnTakeDamage_Range
  (params (Player :type Nazi%20Zombie%20Character%20Object%20Reference) (Damage :type Float%20%28single-precision%29))
  (if (Variables|Default|GetbIsRage)
    (Class|NaziZombieCharacter|IncrementRage Player (CallFunction|CalcualteRecoverableRage Player Damage))))

(event EventBeginPlay
  ;[1 0.6234 0.06443 1 32] Begin Play
  (|CallParentFunction)
  (EventDispatchers|BindEventtoOnTakeAnyDamage (EventDispatchers|CreateEvent :!event Custom|OnTakeDamage))
  (EventDispatchers|BindEventtoOnEnemyDeath (EventDispatchers|CreateEvent :!event Custom|OnDeathEvent))
  (EventDispatchers|BindEventtoOnTakeDamageRange (EventDispatchers|CreateEvent :!event Custom|OnTakeDamage_Range))
  (EventDispatchers|BindEventtoOnTakeDamageMelee (EventDispatchers|CreateEvent :!event Custom|OnTakeDamage_Melee)))

(event EventAttackNotify
  (params (AttackType :type E_BossMoveset%20Enum :default "NewEnumerator0"))
  ;[0 0.4863 1 1 32] Calculate Damage
  (switch Utilities|FlowControl|Switch|SwitchonE_BossMoveset AttackType
    (:NewEnumerator0
      (bind _actor (CallFunction|CalculateTrace 4e+01))
      (Utilities|IsValid _actor
        (:Is%20Valid
          (Game|Damage|ApplyDamage _actor (select (Variables|Default|GetbIsRage) 17.0 12.0) (Variables|Default|GetBP_Controller) self))))
    (:NewEnumerator1
      (bind _actor_2 (CallFunction|CalculateTrace 125.0))
      (Utilities|IsValid _actor_2
        (:Is%20Valid
          (Game|Damage|ApplyDamage _actor_2 (select (Variables|Default|GetbIsRage) 2e+01 15.0) (Variables|Default|GetBP_Controller) self))))
    (:NewEnumerator2
      (CallFunction|CalculateJumpResult))))

(event EventPlaySoundEffect
  (params (AttackType :type E_BossMoveset%20Enum :default "NewEnumerator0"))
  (switch Utilities|FlowControl|Switch|SwitchonE_BossMoveset AttackType
    (:NewEnumerator0
      (CallFunction|PlaySoundEffectFastAttack))
    (:NewEnumerator1
      (CallFunction|PlaySoundEffectStrongAttack))
    (:NewEnumerator2
      ;[1 0 0.001693 1 24] Rage
      (CallFunction|PlaySoundEffectRage))))

(fn ConstructionScript
  (|CallParentFunction))

(fn RotatetoPlayer
  (params (TargetActor :type Actor%20Object%20Reference))
  (Transformation|SetActorRotation (Math|Rotator|MakeRotator 0.0 0.0 (.yaw (Math|Rotator|FindLookatRotation (Transformation|GetActorLocation) (Transformation|GetActorLocation TargetActor)))))
  (return))

(fn GetIsRage
  (return (Variables|Default|GetbIsRage)))

(fn GetIsRageCasting
  (return (Variables|Default|GetbIsRageCasting)))

(fn GetIsJumping
  (return (Variables|Default|GetbIsJumping)))

(fn AttackPlayer
  (params (OtherActor :type Actor%20Object%20Reference))
  (LocalVariables|SetL_PlayRate (select (Variables|Default|GetbIsRage) 1.275 1.0))
  (bind _returnvalue (Animation|Montage|MontagePlay (Components|SkeletalMesh|GetAnimInstance (Variables|Character|GetMesh)) (select (and (<= (Transformation|GetDistanceTo OtherActor) 1.5e+02) (Math|Random|RandomBoolwithWeight (select (Variables|Default|GetbIsRage) 0.25 0.7))) "/Game/BlueprintClasses/Zombies/Animations/Boss_Mutant/AM_Mutant_Punch.AM_Mutant_Punch" "/Game/BlueprintClasses/Zombies/Animations/Boss_Mutant/AM_Mutant_Swiping.AM_Mutant_Swiping") (LocalVariables|GetL_PlayRate) "MontageLength" 0.0 true))
  (return (/ _returnvalue (LocalVariables|GetL_PlayRate))))

(fn CalcualteRecoverableRage
  (params (Player :type Character%20Base%20Object%20Reference) (Damage :type Float%20%28single-precision%29))
  (bind _returnvalue (Class|CharacterBase|GetCurrentWeapon Player))
  (bind _returnvalue_2 (Class|WeaponBase|GetWeaponDamage _returnvalue))
  (bind (_basedamage _rageforheadshot) (Utilities|Struct|BreakWeaponDamage _returnvalue_2))
  (LocalVariables|SetL_Amount (+ (* (/ Damage (Variables|Default|GetMaxHealth)) (* _basedamage 0.1)) (* _rageforheadshot 0.75)))
  (return (select (Variables|/Script/WorldAtWar.CharacterBase|GetbIsRage Player) (* (LocalVariables|GetL_Amount) 0.15) (LocalVariables|GetL_Amount))))

(fn VInterptoMine
  (LocalVariables|SetL_Dist (- (Variables|Default|GetTargetJumpLocation) (Transformation|GetActorLocation)))
  (LocalVariables|SetL_DeltaMove (* (LocalVariables|GetL_Dist) 0.01))
  (Transformation|SetActorLocation (+ (Transformation|GetActorLocation) (LocalVariables|GetL_DeltaMove)) true false)
  (return))

(fn CalculateTrace
  (params (TraceLength :type Float%20%28single-precision%29))
  (LocalVariables|SetL_Start (+ (Transformation|GetActorLocation) (* (Transformation|GetActorForwardVector) 35.0)))
  (bind (_outhit _returnvalue) (Class|KismetSystemLibrary|BoxTraceSingleforObjects (LocalVariables|GetL_Start) (+ (LocalVariables|GetL_Start) (* (Transformation|GetActorForwardVector) TraceLength)) "60.000000,60.000000,80.000000" "0, 0, 0" (Utilities|Array|MakeArray "ObjectTypeQuery3") false 0 "None" true))
  (return _returnvalue (.HitActor (Collision|BreakHitResult _outhit))))

(fn CalculateJumpResult
  (LocalVariables|SetL_Location (+ (- (Transformation|GetActorLocation) "0, 0,100.000000") (* (Transformation|GetActorForwardVector) 4e+02)))
  (Game|Damage|ApplyRadialDamage (select (Variables|Default|GetbIsRage) 3e+01 2e+01) (LocalVariables|GetL_Location) 3.3e+02 0 (Utilities|Array|MakeArray self) 0 0 false "ECC_Pawn")
  (Effects|SpawnEmitteratLocation "/Game/Assets/InfinityBladeEffects/Effects/FX_Monsters/FX_Monster_GolemBot/Mace/P_Mace_Impact_Damage.P_Mace_Impact_Damage" (- (LocalVariables|GetL_Location) "0, 0,70.000000") "0, 0, 0" "1.350000,1.350000,1.350000")
  (return))

(fn PlaySoundEffectStrongAttack
  (bind _bisrage (Variables|Default|GetbIsRage))
  (bind _bisrage_2 (Variables|Default|GetbIsRage))
  (Audio|PlaySoundatLocation "/Game/Audio/Characters/Bosses/Mutant/S_Mutant_StrongAttack_01.S_Mutant_StrongAttack_01" (Transformation|GetActorLocation) "0, 0, 0" (Math|Random|RandomFloatinRange (select _bisrage 1.05 0.8) (select _bisrage 1.25 1.0)) (Math|Random|RandomFloatinRange (select _bisrage_2 1.05 0.8) (select _bisrage_2 1.25 1.0)) 0.0 0 0 0))

(fn PlaySoundEffectFastAttack
  (Audio|PlaySoundatLocation "/Game/Audio/Characters/Bosses/Mutant/S_Mutant_FastAttack.S_Mutant_FastAttack" (Transformation|GetActorLocation) "0, 0, 0" 1.0 (Math|Random|RandomFloatinRange 0.8 1.2) 0.0 0 0 0))

(fn ShouldJumpAgain
  (if (>= (Transformation|GetDistanceTo (Game|GetPlayerCharacter 0)) 4.5e+02)
    (return (Math|Random|RandomBoolwithWeight (Math|Float|Min(Float) (/ 0.1875 (Class|ZombieBase|GetPercentHealth)) 0.45)))
    (else
      (return false))))

(fn PlaySoundEffectRage
  (Audio|PlaySoundatLocation "/Game/Audio/Characters/Bosses/Mutant/S_Mutant_Roaring.S_Mutant_Roaring" (Transformation|GetActorLocation) "0, 0, 0" 1.0 (Math|Random|RandomFloatinRange 0.8 1.2) 0.0 0 0 0)
  (return))

(fn SetLocationAfterJump
  (Animation|Montage|MontageStop (Components|SkeletalMesh|GetAnimInstance (Variables|Character|GetMesh)) 0.0 "/Game/BlueprintClasses/Zombies/Animations/Boss_Mutant/AM_Mutant_Jump_Attack.AM_Mutant_Jump_Attack")
  (bind _output_get (LocalVariables|SetL_ImpactPoint (+ (Transformation|GetActorLocation) (* (Transformation|GetActorForwardVector) 2.2e+02))))
  (Transformation|SetActorLocation _output_get true false)
  (return))