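; Usable prayer place that grants the player one of five random blessings and punishes persistent praying after a refusal.
; ActivateBless broadcasts the random blessing through a dispatcher and shows its colored HUD message.
; RefuseHelp counts failed attempts, repeating one refusal before escalating warnings end in a punishment broadcast and disabled collision.
; MightPray allows prayer only while the place is not desecrated.
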(event Custom|ActivateBless
  (bind _returnvalue (CallFunction|GetRandomBlessing))
  (Default|CallOnBlessingReceived _returnvalue)
  (CallFunction|ShowBlessingMessage _returnvalue))

(event Custom|RefuseHelp
  (bind _result (Math|Integer|IncrementInt (Variables|Default|GetFailureCounter))
    (:%20%20
      (if (> _result 26)
        (switch int (Variables|Default|GetFailureCounter)
          (:27
            (Class|BPIHUD|ShowMessage(Message) (Variables|Default|GetPlayerHUD) "The chill intensified, you can feel the fear inside you. 
\"That's enough, stop it...\"" "(R=0.517708,G=0.448532,B=0.203067,A=1.000000)" 26 2 5.0))
          (:28
            (Class|BPIHUD|ShowMessage(Message) (Variables|Default|GetPlayerHUD) "You feel a wild shiver all over your body, the cold gets to your bones. 
\"Stop it, stop it now...\"" "(R=0.517708,G=0.285140,B=0.164122,A=1.000000)" 26 2 5.0))
          (:29
            (Class|BPIHUD|ShowMessage(Message) (Variables|Default|GetPlayerHUD) "\"Stop this at once, mortal! You are not worthy of blessing!\"" "(R=0.812500,G=0.362696,B=0.000000,A=1.000000)" 30 2 5.0))
          (:30
            (Class|BPIHUD|ShowMessage(Message) (Variables|Default|GetPlayerHUD) "\"So, be it...\"" "(R=0.546875,G=0.000000,B=0.020421,A=1.000000)" 30 2 5.0)
            (Default|CallOnPunishmentIsDeserved)
            (Collision|SetCollisionEnabled (Variables|Default|GetCollisionComp) "NoCollision")))
        (else
          (Class|BPIHUD|ShowMessage(Message) (Variables|Default|GetPlayerHUD) "You begin to recite a prayer and feel a strange chill on your skin, and a thought pops into your head: 
\"You've already made your choice...\"" "(R=0.387500,G=0.335722,B=0.151994,A=1.000000)" 26 2 5.0))))))

(event EventBeginPlay
  (EventDispatchers|AssignOnObjectUsed (EventDispatchers|CreateEvent :!event Custom|ActivateBless))
  (EventDispatchers|BindEventtoOnFailUse (EventDispatchers|CreateEvent :!event Custom|RefuseHelp))
  (Variables|Default|SetPlayerHUD (HUD|GetHUD (Game|GetPlayerController 0))))

(fn ConstructionScript)

(fn MightPray
  (params (Player :type Nazi%20Zombie%20Character%20Object%20Reference))
  (return (not (Variables|Default|GetbDesecrated))))

(fn GetRandomBlessing
  (return (Utilities|Select :Index (Math|Random|RandomIntegerinRange 0 4) :Option%200 "NewEnumerator0" :Option%201 "NewEnumerator1" :Option%202 "NewEnumerator2" :Option%203 "NewEnumerator3" :Option%204 "NewEnumerator4")))

(fn ShowBlessingMessage
  (params (Blessing :type E_Blessings%20Enum :default "NewEnumerator0"))
  (switch Utilities|FlowControl|Switch|SwitchonE_Blessings Blessing
    (:NewEnumerator0
      (Class|BPIHUD|ShowMessage(Message) (Variables|Default|GetPlayerHUD) "Blessing received: Righteous Wrath 
During combat, the character will gradually accumulate rage points" "(R=0.909804,G=0.556047,B=0.113361,A=1.000000)" 26 2 6.0))
    (:NewEnumerator1
      (Class|BPIHUD|ShowMessage(Message) (Variables|Default|GetPlayerHUD) "Blessing received: Divine Protection 
Decreases the damage received by 15%, also the character becomes immune to all negative effects" "(R=0.192157,G=0.337255,B=0.909804,A=1.000000)" 26 2 6.0))
    (:NewEnumerator2
      (Class|BPIHUD|ShowMessage(Message) (Variables|Default|GetPlayerHUD) "Blessing received: Regenration 
During combat, the character will gradually regenerate health points" "(R=0.662745,G=0.909804,B=0.184314,A=1.000000)" 26 2 6.0))
    (:NewEnumerator3
      (Class|BPIHUD|ShowMessage(Message) (Variables|Default|GetPlayerHUD) "Blessing received: The Punishing Hand 
Damage dealt is increased by 20%" "(R=0.862500,G=0.063158,B=0.050313,A=1.000000)" 26 2 6.0))
    (:NewEnumerator4
      (Class|BPIHUD|ShowMessage(Message) (Variables|Default|GetPlayerHUD) "Blessing received: Iron Flesh 
The maximum health reserve is increased by 40%" "(R=0.442842,G=0.862500,B=0.835024,A=1.000000)" 26 2 6.0)))
  (return))