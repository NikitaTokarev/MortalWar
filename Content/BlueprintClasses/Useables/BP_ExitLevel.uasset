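; BP_ExitLevel is a useable level exit whose prompt tells the player to two-finger touch to leave the level.
; On BeginPlay it runs the parent's logic, then sets that UI message.
; Activate makes its collision component block WorldDynamic and starts a spinning-sword particle effect.
; Deactivate only sets that channel back to Ignore, leaving the effect untouched; the level-leaving logic is not in this graph.
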(event Custom|Activate
  (Collision|SetCollisionResponsetoChannel (Variables|Default|GetCollisionComp) "ECC_WorldDynamic" "ECR_Block")
  (Components|Activation|Activate (Variables|Default|GetP_Greystone_Novaborn_SwordSpinning_01) true))

(event Custom|Deactivate
  (Collision|SetCollisionResponsetoChannel (Variables|Default|GetCollisionComp) "ECC_WorldDynamic" "ECR_Ignore"))

(event EventBeginPlay
  (|CallParentFunction)
  (Variables|Default|SetUIMessage (Utilities|Text|MakeLiteralText "Two-finger touch to leave this level")))

(fn ConstructionScript)