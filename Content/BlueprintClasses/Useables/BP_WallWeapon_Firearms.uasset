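; Wall-mounted firearm pickup for a Nazi zombie game, offering variants of the Colt 1911, M1 Carbine and STG44 at a cost.
; The construction script maps the chosen variant to its weapon Blueprint and outline material.
; A dynamic material instance tints the outline's emissive color by variant, unless OtherColor applies a custom color.
; On BeginPlay, after parent logic, it builds the touch prompt from the display name and the player's cost.
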(event EventBeginPlay
  (|CallParentFunction)
  (Class|WallWeapon|ChangeUIMessage))

(event EventChangeUIMessage
  (Variables|Default|SetUIMessage (Utilities|Text|FormatText "Two-finger touch to take {obj} [Cost: {Val}]" (Variables|Default|GetDisplayName) (Class|InteractableBase|GetCost (.AsBP%20Nazi%20Zombie%20Character (Utilities|Casting|CastToBP_NaziZombieCharacter (Game|GetPlayerCharacter 0)))))))

(fn ConstructionScript
  (bind _wallweaponmesh (Variables|Default|GetWallWeaponMesh))
  (Variables|Default|SetWeaponClass (Utilities|Select :Index (Variables|Default|GetWeaponClass_) :NewEnumerator0 "/Game/Weapons/1911/BP_Colt1911.BP_Colt1911_C" :NewEnumerator1 "/Game/Weapons/1911/BP_Colt1911_Silver.BP_Colt1911_Silver_C" :NewEnumerator2 "/Game/Weapons/1911/BP_Colt1911_Rare.BP_Colt1911_Rare_C" :NewEnumerator3 "/Game/Weapons/M1Carbine/BP_M1Carbine.BP_M1Carbine_C" :NewEnumerator4 "/Game/Weapons/M1Carbine/BP_M1Carbine_AncientWeapon.BP_M1Carbine_AncientWeapon_C" :NewEnumerator5 "/Game/Weapons/M1Carbine/BP_M1Carbine_RedWood.BP_M1Carbine_RedWood_C" :NewEnumerator6 "/Game/Weapons/STG44/BP_STG44.BP_STG44_C" :NewEnumerator7 "/Game/Weapons/STG44/BP_STG44_Silver.BP_STG44_Silver_C" :NewEnumerator8 "/Game/Weapons/STG44/BP_STG44_Rare.BP_STG44_Rare_C"))
  (Rendering|Material|SetMaterial (Variables|Default|GetWallWeaponMesh) 0 (Utilities|Select :Index (Variables|Default|GetWeaponClass_) :NewEnumerator0 "/Game/Assets/WallWeapon/MI_WeaponOutlineMaster_Firearm_1911.MI_WeaponOutlineMaster_Firearm_1911" :NewEnumerator1 "/Game/Assets/WallWeapon/MI_WeaponOutlineMaster_Firearm_1911.MI_WeaponOutlineMaster_Firearm_1911" :NewEnumerator2 "/Game/Assets/WallWeapon/MI_WeaponOutlineMaster_Firearm_1911.MI_WeaponOutlineMaster_Firearm_1911" :NewEnumerator3 "/Game/Assets/WallWeapon/MI_WeaponOutlineMaster_Firearm_M1Carbine.MI_WeaponOutlineMaster_Firearm_M1Carbine" :NewEnumerator4 "/Game/Assets/WallWeapon/MI_WeaponOutlineMaster_Firearm_M1Carbine.MI_WeaponOutlineMaster_Firearm_M1Carbine" :NewEnumerator5 "/Game/Assets/WallWeapon/MI_WeaponOutlineMaster_Firearm_M1Carbine.MI_WeaponOutlineMaster_Firearm_M1Carbine" :NewEnumerator6 "/Game/Assets/WallWeapon/MI_WeaponOutlineMaster_Firearm_STG44.MI_WeaponOutlineMaster_Firearm_STG44" :NewEnumerator7 "/Game/Assets/WallWeapon/MI_WeaponOutlineMaster_Firearm_STG44.MI_WeaponOutlineMaster_Firearm_STG44" :NewEnumerator8 "/Game/Assets/WallWeapon/MI_WeaponOutlineMaster_Firearm_STG44.MI_WeaponOutlineMaster_Firearm_STG44"))
  (bind _returnvalue (Rendering|Material|CreateDynamicMaterialInstance _wallweaponmesh 0 (Rendering|Material|GetMaterial _wallweaponmesh 0) "None" :!class /Script/Engine.PrimitiveComponent))
  (if (Variables|Default|GetbOtherColor)
    (Rendering|Material|SetVectorParameterValue _returnvalue "EmissiveColor" (Variables|Default|GetNewColor) :!class /Script/Engine.MaterialInstanceDynamic)
    (else
      (Rendering|Material|SetVectorParameterValue _returnvalue "EmissiveColor" (Utilities|Select :Index (Variables|Default|GetWeaponClass_) :NewEnumerator0 "(R=0.505882,G=0.541176,B=0.600000,A=1.000000)" :NewEnumerator1 "(R=0.078431,G=0.117647,B=0.337255,A=1.000000)" :NewEnumerator2 "(R=1.000000,G=0.094118,B=0.000000,A=1.000000)" :NewEnumerator3 "(R=0.505882,G=0.541176,B=0.600000,A=1.000000)" :NewEnumerator4 "(R=0.078431,G=0.117647,B=0.337255,A=1.000000)" :NewEnumerator5 "(R=1.000000,G=0.094118,B=0.000000,A=1.000000)" :NewEnumerator6 "(R=0.505882,G=0.541176,B=0.600000,A=1.000000)" :NewEnumerator7 "(R=0.078431,G=0.117647,B=0.337255,A=1.000000)" :NewEnumerator8 "(R=1.000000,G=0.094118,B=0.000000,A=1.000000)") :!class /Script/Engine.MaterialInstanceDynamic))))