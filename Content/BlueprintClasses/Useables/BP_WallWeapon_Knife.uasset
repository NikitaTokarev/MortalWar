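; Wall-mounted knife pickup that offers one of three melee weapons (Knife, SilverBlade, HuntingKnife) for a cost.
; The construction script maps the WeaponClass setting to the knife Blueprint and a special color.
; It also creates a dynamic material on the wall mesh, tinting its emissive color per variant unless an override color is enabled.
; On BeginPlay it builds the two-finger touch prompt from the display name and cost.
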(event EventBeginPlay
  (|CallParentFunction)
  (Class|WallWeapon|ChangeUIMessage))

(event EventChangeUIMessage
  (Variables|Default|SetUIMessage (Utilities|Text|FormatText "Two-finger touch to take {obj} [Cost: {Val}]" (Variables|Default|GetDisplayName) (Class|InteractableBase|GetCost))))

(fn ConstructionScript
  (bind _wallweaponmesh (Variables|Default|GetWallWeaponMesh))
  (Variables|Default|SetKnifeClass (Utilities|Select :Index (Variables|Default|GetWeaponClass) :NewEnumerator0 "/Game/Weapons/Knife/Default/BP_Knife.BP_Knife_C" :NewEnumerator1 "/Game/Weapons/Knife/SilverKnife/BP_SilverBlade.BP_SilverBlade_C" :NewEnumerator2 "/Game/Weapons/Knife/HuntingKnife/BP_HuntingKnife.BP_HuntingKnife_C"))
  (CallFunction|SetSpecialColor (Variables|Default|GetWeaponClass))
  (bind _returnvalue (Rendering|Material|CreateDynamicMaterialInstance _wallweaponmesh 0 (Rendering|Material|GetMaterial _wallweaponmesh 0) "None" :!class /Script/Engine.PrimitiveComponent))
  (if (Variables|Default|GetbOtherColor)
    (Rendering|Material|SetVectorParameterValue _returnvalue "EmissiveColor" (Variables|Default|GetNewColor) :!class /Script/Engine.MaterialInstanceDynamic)
    (else
      (Rendering|Material|SetVectorParameterValue _returnvalue "EmissiveColor" (Utilities|Select :Index (Variables|Default|GetWeaponClass) :NewEnumerator0 "(R=0.000000,G=0.000000,B=0.000000,A=1.000000)" :NewEnumerator1 "(R=0.078431,G=0.117647,B=0.337255,A=1.000000)" :NewEnumerator2 "(R=1.000000,G=0.094118,B=0.000000,A=1.000000)") :!class /Script/Engine.MaterialInstanceDynamic))))

(fn SetSpecialColor
  (params (Quality :type E_Weapon_Melee%20Enum :default "NewEnumerator0"))
  (Variables|Default|SetbSpecialColor true)
  (Variables|Default|SetSpecialColor (Utilities|Select :Index Quality :NewEnumerator0 "(R=1.000000,G=1.000000,B=1.000000,A=1.000000)" :NewEnumerator1 "(R=0.180392,G=0.376471,B=0.533333,A=1.000000)" :NewEnumerator2 "(R=0.964706,G=0.427451,B=0.003922,A=1.000000)"))
  (return))