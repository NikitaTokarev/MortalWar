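; BP_MysteryBox is a useable mystery box that shows a two-finger touch prompt to open it, including the cost when above zero.
; On BeginPlay it creates dynamic instances of both mesh materials, then a looping timer fades it in by raising their OpacityMask parameter.
; StartDisappearing waits briefly, then a second timer lowers the mask until it drops below zero, without destroying the actor.
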(event Custom|Appearing
  (bind _output_get (Variables|Default|SetOpacityMask (+ (Variables|Default|GetOpacityMask) 0.0125)))
  (Rendering|Material|SetScalarParameterValue (Variables|Default|GetMI_First) "OpacityMask" _output_get :!class /Script/Engine.MaterialInstanceDynamic)
  (if (Math|Float|NearlyEqual(Float) _output_get 0.5 1e-06)
    (Utilities|Time|ClearandInvalidateTimerbyHandle (stale EventBeginPlay _returnvalue_2))))

(event Custom|Disappearing
  (bind _output_get (Variables|Default|SetOpacityMask (- (Variables|Default|GetOpacityMask) 0.025)))
  (Rendering|Material|SetScalarParameterValue (Variables|Default|GetMI_First) "OpacityMask" _output_get :!class /Script/Engine.MaterialInstanceDynamic)
  (if (< _output_get 0.0)
    (Utilities|Time|ClearandInvalidateTimerbyHandle (stale EventStartDisappearing _returnvalue))))

(event EventBeginPlay
  (bind _returnvalue (Class|InteractableBase|GetCost))
  (|CallParentFunction)
  (Variables|Default|SetUIMessage (select (> _returnvalue 0) (Utilities|Text|FormatText "Two-finger touch to open {obj} [Cost: {Cost}]" (Variables|Default|GetDisplayName) _returnvalue) (Utilities|Text|FormatText "Two-finger touch to open {obj}" (Variables|Default|GetDisplayName))))
  (CallFunction|InitMaterials)
  (bind _returnvalue_2 (Utilities|Time|SetTimerbyEvent (delegate Custom|Appearing) 0.05 true)))

(event EventStartDisappearing
  (Utilities|FlowControl|Delay 0.95)
  (bind _returnvalue (Utilities|Time|SetTimerbyEvent (delegate Custom|Disappearing) 0.05 true)))

(fn ConstructionScript)

(fn InitMaterials
  (bind _mysteryboxmesh (Variables|Default|GetMysteryBoxMesh))
  (bind _returnvalue (Rendering|Material|CreateDynamicMaterialInstance _mysteryboxmesh 0 (Rendering|Material|GetMaterial _mysteryboxmesh 0) "None" :!class /Script/Engine.PrimitiveComponent))
  (Variables|Default|SetMI_First _returnvalue)
  (bind _returnvalue_2 (Rendering|Material|CreateDynamicMaterialInstance _mysteryboxmesh 1 (Rendering|Material|GetMaterial _mysteryboxmesh 1) "None" :!class /Script/Engine.PrimitiveComponent))
  (Variables|Default|SetMI_Second _returnvalue_2))