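; Lootable weapon pickup that displays the model, name and two-finger-touch equip prompt for its assigned weapon class.
; SetViewModel runs SetupMesh, builds the prompt text, then enables collision overlap events after a short delay.
; SetupMesh uses parent-class checks for firearms and exact-class checks for blades to choose and position a skeletal or static mesh.
; Exact firearm variants set names, with Silver and Rare variants adding material overrides and special colors.
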(event EventBeginPlay)

(event Collision|EventActorBeginOverlap
  (params (OtherActor :type Actor%20Object%20Reference)))

(event EventTick
  (params (DeltaSeconds :type Float%20%28single-precision%29)))

(event EventSetViewModel
  (CallFunction|SetupMesh)
  (Variables|Default|SetUIMessage (Utilities|Text|FormatText "Two-finger touch to equip {obj}" (Variables|Default|GetDisplayName)))
  (Utilities|FlowControl|Delay 1.0)
  (Variables|/Script/Engine.PrimitiveComponent|SetbGenerateOverlapEvents (Variables|Default|GetCollisionComponent) true))

(fn ConstructionScript)

(fn SetupMesh
  (Utilities|CheckWeaponParentClass "/Game/Weapons/1911/BP_Colt1911.BP_Colt1911_C"
    (:True
      (Class|SkinnedMeshComponent|SetSkeletalMesh (Variables|Default|GetSkeletalMesh) "/Game/Weapons/1911/Meshes/1911.1911" true)
      (CallFunction|SetFireArmsMaterial "NewEnumerator0")
      (CallFunction|HideMagazine)
      (CallFunction|SetRelativeLocation&Scale "5.000000,2.000000, 0" "1.450000,1.450000,1.450000" (Variables|Default|GetSkeletalMesh))
      (return))
    (:False
      (Utilities|CheckWeaponParentClass "/Game/Weapons/M1Carbine/BP_M1Carbine.BP_M1Carbine_C"
        (:True
          (Class|SkinnedMeshComponent|SetSkeletalMesh (Variables|Default|GetSkeletalMesh) "/Game/Weapons/M1Carbine/Meshes/M1_Carbine.M1_Carbine" true)
          (CallFunction|SetFireArmsMaterial "NewEnumerator3")
          (CallFunction|SetRelativeLocation&Scale "28.000000,0.000000, 0" "1.200000,1.200000,1.200000" (Variables|Default|GetSkeletalMesh))
          (return))
        (:False
          (Utilities|CheckWeaponParentClass "/Game/Weapons/STG44/BP_STG44.BP_STG44_C"
            (:True
              (Class|SkinnedMeshComponent|SetSkeletalMesh (Variables|Default|GetSkeletalMesh) "/Game/Weapons/STG44/Meshes/SK_Stg44.SK_Stg44" true)
              (CallFunction|SetFireArmsMaterial "NewEnumerator6")
              (CallFunction|HideMagazine)
              (CallFunction|SetRelativeLocation&Scale "20.000000,-3.000000, 0" "1.200000,1.200000,1.200000" (Variables|Default|GetSkeletalMesh))
              (return))
            (:False
              (Utilities|CheckWeaponClass "/Game/Weapons/Knife/Default/BP_Knife.BP_Knife_C"
                (:True
                  (Components|StaticMesh|SetStaticMesh (Variables|Default|GetStaticMesh) "/Game/Weapons/Knife/Default/SM_DefaultKnife.SM_DefaultKnife")
                  (Variables|Default|SetDisplayName "Knife")
                  (CallFunction|SetRelativeLocation&Scale "15.000000, 0, 0" "1.650000,1.650000,1.650000" (Variables|Default|GetStaticMesh))
                  (return))
                (:False
                  (Utilities|CheckWeaponClass "/Game/Weapons/Knife/SilverKnife/BP_SilverBlade.BP_SilverBlade_C"
                    (:True
                      (Components|StaticMesh|SetStaticMesh (Variables|Default|GetStaticMesh) "/Game/Weapons/Knife/SilverKnife/SM_SilverBlade.SM_SilverBlade")
                      (Variables|Default|SetDisplayName "Silver Dagger")
                      (CallFunction|SetRelativeLocation&Scale "30.000000, 0, 0" "1.650000,1.650000,1.650000" (Variables|Default|GetStaticMesh))
                      (CallFunction|SetSpecialColor "NewEnumerator1")
                      (return))
                    (:False
                      (Utilities|CheckWeaponClass "/Game/Weapons/Knife/HuntingKnife/BP_HuntingKnife.BP_HuntingKnife_C"
                        (:True
                          (Variables|Default|SetDisplayName "Hunting Blade")
                          (Components|StaticMesh|SetStaticMesh (Variables|Default|GetStaticMesh) "/Game/Weapons/Knife/HuntingKnife/SM_HuntingKnife.SM_HuntingKnife")
                          (CallFunction|SetRelativeLocation&Scale "30.000000, 0, 0" "1.650000,1.650000,1.650000" (Variables|Default|GetStaticMesh))
                          (CallFunction|SetSpecialColor "NewEnumerator2")
                          (return))
                        (:False
                          (Variables|Default|SetDisplayName "???")
                          (return))))))))))))))

(fn GetFireArmsMaterial
  (return 0))

(fn GetMeleeMaterial
  (return 0))

(fn SetRelativeLocation&Scale
  (params (NewLocation :type Vector) (NewScale3D :type Vector :default "1.000000,1.000000,1.000000") (Target :type Scene%20Component%20Object%20Reference))
  (Transformation|SetRelativeLocation Target NewLocation false false)
  (Transformation|SetRelativeScale3D Target NewScale3D)
  (return))

(fn HideMagazine
  (Components|SkinnedMesh|HideBonebyName (Variables|Default|GetSkeletalMesh) "Magazine2" "PBO_None")
  (return))

(fn SetFireArmsMaterial
  (params (Type :type E_Weapon_Firearms%20Enum :default "NewEnumerator0"))
  (switch Utilities|FlowControl|Switch|SwitchonE_Weapon_Firearms Type
    (:NewEnumerator0
      (Utilities|CheckWeaponClass "/Game/Weapons/1911/BP_Colt1911.BP_Colt1911_C"
        (:True
          (Variables|Default|SetDisplayName "M1911")
          (return))
        (:False
          (Utilities|CheckWeaponClass "/Game/Weapons/1911/BP_Colt1911_Rare.BP_Colt1911_Rare_C"
            (:True
              (Variables|Default|SetDisplayName "Shooter's Gun")
              (Rendering|Material|SetMaterial (Variables|Default|GetSkeletalMesh) 0 "/Game/Weapons/1911/Textures/MI_Colt1911_Rare.MI_Colt1911_Rare")
              (CallFunction|SetSpecialColor "NewEnumerator2")
              (return))
            (:False
              (Utilities|CheckWeaponClass "/Game/Weapons/1911/BP_Colt1911_Silver.BP_Colt1911_Silver_C"
                (:True
                  (Variables|Default|SetDisplayName "Silver Colt")
                  (Rendering|Material|SetMaterial (Variables|Default|GetSkeletalMesh) 0 "/Game/Weapons/1911/Textures/MI_Colt1911_Silver.MI_Colt1911_Silver")
                  (CallFunction|SetSpecialColor "NewEnumerator1")
                  (return))
                (:False
                  (return))))))))
    (:NewEnumerator3
      (Utilities|CheckWeaponClass "/Game/Weapons/M1Carbine/BP_M1Carbine.BP_M1Carbine_C"
        (:True
          (Variables|Default|SetDisplayName "M1 Carbine")
          (return))
        (:False
          (Utilities|CheckWeaponClass "/Game/Weapons/M1Carbine/BP_M1Carbine_AncientWeapon.BP_M1Carbine_AncientWeapon_C"
            (:True
              (Variables|Default|SetDisplayName "Ancient Gun")
              (Rendering|Material|SetMaterial (Variables|Default|GetSkeletalMesh) 0 "/Game/Weapons/M1Carbine/Textures/MI_M1Carbine_Ancient.MI_M1Carbine_Ancient")
              (CallFunction|SetSpecialColor "NewEnumerator1")
              (return))
            (:False
              (Utilities|CheckWeaponClass "/Game/Weapons/M1Carbine/BP_M1Carbine_RedWood.BP_M1Carbine_RedWood_C"
                (:True
                  (Variables|Default|SetDisplayName "Elite Rifle")
                  (Rendering|Material|SetMaterial (Variables|Default|GetSkeletalMesh) 0 "/Game/Weapons/M1Carbine/Textures/M_M1Carbine_RedWood.M_M1Carbine_RedWood")
                  (CallFunction|SetSpecialColor "NewEnumerator2")
                  (return))
                (:False
                  (return))))))))
    (:NewEnumerator6
      (Utilities|CheckWeaponClass "/Game/Weapons/STG44/BP_STG44.BP_STG44_C"
        (:True
          (Variables|Default|SetDisplayName "STG 44")
          (return))
        (:False
          (Utilities|CheckWeaponClass "/Game/Weapons/STG44/BP_STG44_Silver.BP_STG44_Silver_C"
            (:True
              (Variables|Default|SetDisplayName "Assault Rifle")
              (Rendering|Material|SetMaterial (Variables|Default|GetSkeletalMesh) 0 "/Game/Weapons/STG44/Textures/MI_STG44_Silver.MI_STG44_Silver")
              (CallFunction|SetSpecialColor "NewEnumerator1")
              (return))
            (:False
              (Utilities|CheckWeaponClass "/Game/Weapons/STG44/BP_STG44_Rare.BP_STG44_Rare_C"
                (:True
                  (Variables|Default|SetDisplayName "MP 43")
                  (Rendering|Material|SetMaterial (Variables|Default|GetSkeletalMesh) 0 "/Game/Weapons/STG44/Textures/MI_STG44_Rare.MI_STG44_Rare")
                  (CallFunction|SetSpecialColor "NewEnumerator2")
                  (return))
                (:False
                  (return))))))))))

(fn SetSpecialColor
  (params (Quality :type E_WeaponsQuality%20Enum :default "NewEnumerator1"))
  (Variables|Default|SetbSpecialColor true)
  (Variables|Default|SetSpecialColor (Utilities|Select :Index Quality :NewEnumerator0 "" :NewEnumerator1 "(R=0.182222,G=0.378455,B=0.533333,A=1.000000)" :NewEnumerator2 "(R=0.775000,G=0.344004,B=0.005277,A=1.000000)"))
  (return))