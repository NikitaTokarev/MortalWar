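; AI controller for zombies that chases a living player and triggers melee attacks on reaching them.
; On the server, online games pick the nearest living BP_NaziZombieCharacter using a looping retarget timer, while offline games target the first player.
; AIMoveTo success leads to an attack, multicast through BP_ZombieBase online or played directly offline, and failure retries the search.
; Retargeting pauses during online attacks and resumes afterward.
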(event Custom|Attack
  (params (Target :type Actor%20Object%20Reference))
  (bind _returnvalue (Pawn|GetControlledPawn))
  (bind _returnvalue_2 (Pawn|GetControlledPawn))
  (bind _returnvalue_3 (Pawn|GetControlledPawn))
  (bind _returnvalue_4 (Transformation|GetActorRotation _returnvalue_2))
  (bind (_roll _pitch) (Math|Rotator|BreakRotator _returnvalue_4))
  (Transformation|SetActorRotation _returnvalue_3 (Math|Rotator|MakeRotator _roll _pitch (.Yaw (Math|Rotator|BreakRotator (Math|Rotator|FindLookatRotation (Transformation|GetActorLocation _returnvalue_3) (Transformation|GetActorLocation Target))))))
  (bind _returnvalue_5 (Class|BPIEnemyBase|GetZombieRef(Message) _returnvalue))
  (bind _returnvalue_6 (Class|BPIEnemyBase|GetAttackMontage(Message) _returnvalue))
  (bind _returnvalue_7 (Animation|PlayAnimMontage _returnvalue_5 _returnvalue_6 1.0 "None"))
  (Networking|SwitchHasAuthority
    (:Authority
      (if (Variables|Default|GetbIsOnline)
        (Utilities|Time|PauseTimerbyHandle (Variables|Default|GetTH_FindClosestTarget)))
      (Utilities|FlowControl|Delay _returnvalue_7)
      (CallFunction|FindClosestEnemy)
      (if (Variables|Default|GetbIsOnline)
        (Utilities|Time|UnpauseTimerbyHandle (Variables|Default|GetTH_FindClosestTarget))))))

(event Custom|MoveToPlayer
  (AI|AIMoveTo (Pawn|GetControlledPawn) "0, 0, 0" (Variables|Default|GetClosestPlayer) 45.0 false
    (:OnSuccess
      (bind (_dead _returnvalue) (Class|BPIEnemyBase|CanAttack(Message) (Pawn|GetControlledPawn)))
      (if (not _dead)
        (if _returnvalue
          (if (Variables|Default|GetbIsOnline)
            (Utilities|Time|PauseTimerbyHandle (Variables|Default|GetTH_FindClosestTarget))
            (bind _asbp_zombie_base (Utilities|Casting|CastToBP_ZombieBase (Pawn|GetControlledPawn)))
            (Default|MultiPrepareAttack _asbp_zombie_base (Variables|Default|GetClosestPlayer))
            (else
              (CallFunction|Attack (Variables|Default|GetClosestPlayer)))))))
    (:OnFail
      (CallFunction|FindClosestEnemy))))

(event Custom|FindClosestEnemy
  (if (Variables|Default|GetbIsOnline)
    (Variables|Default|SetClosestPlayer 0)
    (Variables|Default|SetBestDistance 29999.0)
    (bind _outactors (Actor|GetAllActorsOfClass "/Game/BlueprintClasses/Player/BP_NaziZombieCharacter.BP_NaziZombieCharacter_C"))
    (for _array_element _outactors
      (if (not (Class|NaziZombieCharacter|GetIsDead _array_element))
        (if (< (Transformation|GetDistanceTo _array_element) (Variables|Default|GetBestDistance))
          (Variables|Default|SetClosestPlayer _array_element)
          (Variables|Default|SetBestDistance (Transformation|GetDistanceTo _array_element))))))
  (Utilities|IsValid (Variables|Default|GetClosestPlayer)
    (:Is%20Valid
      (if (not (Class|NaziZombieCharacter|GetIsDead (Variables|Default|GetClosestPlayer)))
        (CallFunction|MovetoPlayer)))))

(event EventBeginPlay
  (Networking|SwitchHasAuthority
    (:Authority
      (Utilities|FlowControl|Delay 0.4)
      (if (Class|BlueprintFunctionLibraryMisc|IsOnline self)
        (Variables|Default|SetbIsOnline true)
        (bind _returnvalue (Utilities|Time|SetTimerbyEvent (EventDispatchers|CreateEvent :!event Custom|FindClosestEnemy) 2.0 true))
        (Variables|Default|SetTH_FindClosestTarget _returnvalue)
        (else
          (bind _returnvalue_2 (Class|BPIPlayerCharacter|GetPlayerRef(Message) (Game|GetPlayerCharacter 0)))
          (Variables|Default|SetClosestPlayer _returnvalue_2)))
      (CallFunction|FindClosestEnemy))))

(event EventAttackFinished
  (Utilities|Time|UnpauseTimerbyHandle (Variables|Default|GetTH_FindClosestTarget))
  (CallFunction|FindClosestEnemy))

(fn ConstructionScript)