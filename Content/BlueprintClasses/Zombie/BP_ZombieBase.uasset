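; Base zombie enemy Blueprint that handles a temporary anger state, melee attack animation and the roar sound.
; On the server, taking damage can randomly trigger anger, doubling damage and raising walk speed via multicast until a timer reverts both.
; Attack preparation turns the zombie toward its target and plays a random montage, then the server notifies the controller once it finishes.
; The roar stops on death or an explicit shutdown event.
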(event Custom|OnEnemyDeath_Event_0
  (Audio|Components|Audio|Stop (Variables|Default|GetS_Zombie_Roar_Cue)))

(event Custom|OnTakeAnyDamage_Event_0
  (params (DamagedActor :type Actor%20Object%20Reference) (Damage :type Float%20%28single-precision%29) (DamageType :type Damage%20Type%20Object%20Reference) (InstigatedBy :type Controller%20Object%20Reference) (DamageCauser :type Actor%20Object%20Reference))
  (if (not (Variables|Default|GetbIsAnger))
    (if (Math|Random|RandomBoolwithWeight 0.33)
      (Variables|Default|SetbIsAnger true)
      (Variables|Default|SetDamage (* (Class|ZombieBase|GetDamage) 2.0))
      (CallFunction|MultiChangeMaxSpeed 3.5e+02)
      (Utilities|Time|SetTimerbyEvent (delegate Custom|AngerFinished) 15.0))))

(event Custom|Multi_ChangeMaxSpeed
  (params (MaxSpeed :type Float%20%28single-precision%29))
  (Variables|/Script/Engine.CharacterMovementComponent|SetMaxWalkSpeed (Variables|Character|GetCharacterMovement) MaxSpeed))

(event Custom|AngerFinished
  (Variables|Default|SetbIsAnger false)
  (Variables|Default|SetDamage (* (Class|ZombieBase|GetDamage) 0.5))
  (CallFunction|MultiChangeMaxSpeed 1.5e+02))

(event Custom|Multi_PrepareAttack
  (params (Target :type Actor%20Object%20Reference))
  (bind _returnvalue (Transformation|GetActorRotation))
  (bind (_roll _pitch) (Math|Rotator|BreakRotator _returnvalue))
  (Transformation|SetActorRotation (Math|Rotator|MakeRotator _roll _pitch (.Yaw (Math|Rotator|BreakRotator (Math|Rotator|FindLookatRotation (Transformation|GetActorLocation) (Transformation|GetActorLocation Target))))))
  (bind _returnvalue_2 (CallFunction|GetAttackMontage))
  (bind _returnvalue_3 (Animation|PlayAnimMontage _returnvalue_2 1.0 "None"))
  (Networking|SwitchHasAuthority
    (:Authority
      (Utilities|FlowControl|Delay _returnvalue_3)
      (Class|BPIAIController|AttackFinished(Message) (Pawn|GetController)))))

(event EventBeginPlay
  (|CallParentFunction)
  (EventDispatchers|AssignOnEnemyDeath (delegate Custom|OnEnemyDeath_Event_0))
  (Networking|SwitchHasAuthority
    (:Authority
      (EventDispatchers|AssignOnTakeAnyDamage (delegate Custom|OnTakeAnyDamage_Event_0)))))

(event EventShutdownSound
  (Audio|Components|Audio|Stop (Variables|Default|GetS_Zombie_Roar_Cue)))

(fn ConstructionScript)

(fn GetAttackMontage
  (return (.OutItem (Utilities|Array|Random (Variables|Default|GetAttackMontages)))))

(fn GetZombieRef
  (return self))