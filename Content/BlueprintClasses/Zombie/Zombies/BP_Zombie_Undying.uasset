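; Undying zombie variant that has a random chance on its first death to come back as a crawler, and dies for good on the next.
; Die picks between Multi_Resurrection and Multi_Death, both of which play the death montage.
; Resurrection uses timed delays to toggle collision, hide briefly during the switch, and set crawl speed and attack, with authority handling revival, forward offset and retargeting.
; CanAttack blocks attacks while dead or resurrecting.
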(event Custom|Multi_Resurrection
  (bind _returnvalue (Transformation|GetActorForwardVector))
  (bind _attackmontages (Variables|Default|GetAttackMontages))
  (Audio|Components|Audio|Stop (Variables|Default|GetS_Zombie_Roar_Cue))
  (Variables|/Script/Engine.CharacterMovementComponent|SetRotationRate (Variables|Character|GetCharacterMovement) "0, 0, 0")
  (Variables|Default|SetbPrepareToResurrect true)
  (Collision|SetCollisionResponsetoChannel (Variables|Character|GetMesh) "ECC_GameTraceChannel2" "ECR_Ignore")
  (Collision|SetCollisionResponsetoChannel (Variables|Default|GetCapsuleComponent) "ECC_Pawn" "ECR_Ignore")
  (Variables|/Script/Engine.CharacterMovementComponent|SetMaxWalkSpeed (Variables|Character|GetCharacterMovement) 0.0)
  (bind _returnvalue_2 (Animation|Montage|MontagePlay (Components|SkeletalMesh|GetAnimInstance (Variables|Character|GetMesh)) "/Game/BlueprintClasses/Zombie/Animations/Zombie_Undying/AM_Zombie_Undying_Death.AM_Zombie_Undying_Death" 1.0 "MontageLength" 0.0 true))
  (Utilities|FlowControl|Delay (- _returnvalue_2 0.5))
  (Collision|SetCollisionResponsetoChannel (Variables|Default|GetCapsuleComponent) "ECC_Pawn" "ECR_Block")
  (Networking|SwitchHasAuthority
    (:Authority
      (Utilities|FlowControl|Delay 0.5)
      (Class|ZombieBase|Resurrect)
      (Transformation|AddActorWorldOffset (Math|Vector|MakeVector (* (.x _returnvalue) 1e+02) (* (.y _returnvalue) 1e+02) 0.0)))
    (:Remote
      _))
  (Rendering|SetActorHiddenInGame true)
  (Variables|Default|SetbIsResurrected true)
  (Default|CallOnResurrecting)
  (Utilities|FlowControl|Delay 0.05)
  (Rendering|SetActorHiddenInGame false)
  (Utilities|FlowControl|Delay 0.45)
  (Collision|SetCollisionResponsetoChannel (Variables|Character|GetMesh) "ECC_GameTraceChannel2" "ECR_Block")
  (Utilities|FlowControl|Delay 1.3)
  (Variables|/Script/Engine.CharacterMovementComponent|SetMaxWalkSpeed (Variables|Character|GetCharacterMovement) 1.4e+02)
  (Utilities|Array|Clear _attackmontages)
  (Utilities|Array|Add _attackmontages "/Game/BlueprintClasses/Zombie/Animations/Zombie_Undying/AM_Zombie_Undying_Crawl_Attack.AM_Zombie_Undying_Crawl_Attack")
  (Variables|Default|SetbPrepareToResurrect false)
  (Variables|/Script/Engine.CharacterMovementComponent|SetRotationRate (Variables|Character|GetCharacterMovement) "0,290.000000, 0")
  (Audio|Components|Audio|Play (Variables|Default|GetS_Zombie_Roar_Cue) 0.0)
  (Networking|SwitchHasAuthority
    (:Authority
      (bind _asbp_aicontroller_zombie (Utilities|Casting|CastToBP_AIController_Zombie (Pawn|GetController)))
      (Default|FindClosestEnemy _asbp_aicontroller_zombie))))

(event Custom|Multi_Death
  (Audio|Components|Audio|Stop (Variables|Default|GetS_Zombie_Roar_Cue))
  (Variables|Default|SetbPrepareToResurrect false)
  (Variables|/Script/Engine.CharacterMovementComponent|SetMaxWalkSpeed (Variables|Character|GetCharacterMovement) 0.0)
  (Collision|SetCollisionResponsetoChannel (Variables|Character|GetMesh) "ECC_GameTraceChannel2" "ECR_Ignore")
  (Animation|PlayAnimMontage "/Game/BlueprintClasses/Zombie/Animations/Zombie_Undying/AM_Zombie_Undying_Death.AM_Zombie_Undying_Death" 1.0 "None"))

(event EventBeginPlay
  (|CallParentFunction) ; This node is disabled and will not be called.\nDrag off pins to build functionality.
)

(event EventDie
  (if (Variables|Default|GetbIsResurrected)
    (Variables|Default|SetbPrepareToResurrect true)
    (|CallParentFunction)
    (elif (Math|Random|RandomBoolwithWeight (Variables|ZombieBase|GetRessurectChance))
      (CallFunction|MultiResurrection)
      (else
        (CallFunction|MultiDeath)
        (Utilities|FlowControl|Delay 1.0)
        (|CallParentFunction)))))

(fn ConstructionScript
  (|CallParentFunction))

(fn CanAttack
  (return (Variables|Default|GetbIsDead) (and (not (Variables|Default|GetbIsDead)) (not (Variables|Default|GetbPrepareToResurrect)))))