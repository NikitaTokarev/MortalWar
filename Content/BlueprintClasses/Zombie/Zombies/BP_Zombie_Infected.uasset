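; Infected zombie variant that can pass a disease to players it hits.
; On BeginPlay it runs the parent logic and binds a Disease handler to the attack-success event.
; The handler skips players already infected, then rolls a weighted chance from InfectedChance and calls the player's ServerImposeDisease with a fixed duration and damage.
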(event Custom|Disease
  (params (Player :type BP%20Nazi%20Zombie%20Character%20Object%20Reference))
  (if (not (Variables|/Script/WorldAtWar.NaziZombieCharacter|GetbIsInfected Player))
    (if (Math|Random|RandomBoolwithWeight (Variables|ZombieBase|GetInfectedChance))
      (Class|NaziZombieCharacter|ServerImposeDisease Player 1e+01 3.0))))

(event EventBeginPlay
  (|CallParentFunction)
  (EventDispatchers|BindEventtoOnAttackSuccessfully (delegate Custom|Disease)))

(fn ConstructionScript
  (|CallParentFunction))