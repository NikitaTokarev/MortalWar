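; Base zombie character Blueprint providing networked melee attacks and death cleanup.
; Multi_PrepareAttack turns the zombie toward its target and plays a random attack montage, then the server waits out its length and notifies the controller.
; CalculateAttackResult halts AI movement and runs a short server-side forward line trace, damaging any BP_NaziZombieCharacter hit.
; On death, the roar sound and montage slot stop.
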(event Custom|OnEnemyDeath_Event_0
  (Audio|Components|Audio|Stop (Variables|Default|GetS_Zombie_Roar_Cue))
  (Class|AnimInstance|StopSlotAnimation (Components|SkeletalMesh|GetAnimInstance (Variables|Character|GetMesh)) 0.001 "DefaultSlot"))

(event Custom|CalculateAttackResult
  (bind _returnvalue (Transformation|GetActorLocation))
  (bind _self self)
  (bind _returnvalue_2 (AI|GetAIController _self))
  (Utilities|IsValid _returnvalue_2
    (:Is%20Valid
      (AI|Navigation|StopMovement _returnvalue_2)
      (Networking|SwitchHasAuthority
        (:Authority
          (bind _outhit (Collision|LineTraceByChannel _returnvalue (+ _returnvalue (* (Transformation|GetActorForwardVector) 1.2e+02)) "TraceTypeQuery1" false 0 "None"))
          (if (.bBlockingHit (Collision|BreakHitResult _outhit))
            (bind _asbp_nazi_zombie_character (Utilities|Casting|CastToBP_NaziZombieCharacter (.HitActor (Collision|BreakHitResult _outhit))))
            (Game|Damage|ApplyDamage _asbp_nazi_zombie_character (Class|ZombieBase|GetDamage) 0 0)))))))

(event Custom|Multi_PrepareAttack
  (params (Target :type Actor%20Object%20Reference))
  (bind _returnvalue (Transformation|GetActorRotation))
  (bind (_roll _pitch) (Math|Rotator|BreakRotator _returnvalue))
  (Transformation|SetActorRotation (Math|Rotator|MakeRotator _roll _pitch (.Yaw (Math|Rotator|BreakRotator (Math|Rotator|FindLookatRotation (Transformation|GetActorLocation) (Transformation|GetActorLocation Target))))))
  (bind _returnvalue_2 (CallFunction|GetAttackMontage))
  (bind _returnvalue_3 (Animation|PlayAnimMontage _returnvalue_2 1.0 "None"))
  (Networking|SwitchHasAuthority
    (:Authority
      (Utilities|FlowControl|Delay _returnvalue_3)
      (Class|BPIAIController|AttackFinished(Message) (Pawn|GetController)))))

(event EventBeginPlay
  (|CallParentFunction)
  (EventDispatchers|AssignOnEnemyDeath (delegate Custom|OnEnemyDeath_Event_0)))

(event EventShutdownSound
  (Audio|Components|Audio|Stop (Variables|Default|GetS_Zombie_Roar_Cue)))

(fn ConstructionScript)

(fn CanAttack
  (bind _bisdead (Variables|Default|GetbIsDead))
  (return _bisdead (not _bisdead)))

(fn GetAttackMontage
  (return (.OutItem (Utilities|Array|Random (Variables|Default|GetAttackMontages)))))

(fn GetZombieRef
  (return self))